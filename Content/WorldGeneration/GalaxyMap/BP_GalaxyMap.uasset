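; Galaxy map actor that procedurally builds the galaxy's star systems and spawns a BP_GalaxyMap_StarSystem for each.
; BeginPlay seeds a random stream with a polynomial hash of the galaxy name, though the loop reads only index 0's character.
; The stream picks unique DT_StarSystemNames entries and polar positions within GalaxyRadius, then saves the map.
; The branch that loads a saved map is hard-wired off, so every play regenerates it.
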(event EventBeginPlay
  (bind (_galaxyfound _systemdata _galaxytime) (CallFunction|LoadGalaxyMap))
  (if false
    (Variables|Default|SetStarSystemData _systemdata)
    (Variables|Default|SetGalaxy%20Time _galaxytime)
    (else
      (CallFunction|GenerateRandomStreamSeed)
      (CallFunction|GenerateSystemData)))
  (CallFunction|SpawnGalaxyMap))

(fn ConstructionScript
  (Components|Sphere|SetSphereRadius (Variables|Default|GetSphere) (Variables|Default|GetGalaxyRadius) true))

(fn GenerateRandomStreamSeed
  (bind _asvoidsingergameinstance (CallFunction|GetVoidsingerGameInstance))
  (bind _galaxyname (Variables|/Game/GameInfrastructure/BP_Voidsinger_GameInstance.BP_Voidsinger_GameInstance_C|GetGalaxyName _asvoidsingergameinstance))
  ;[0 0 1] Uses a polynomial rolling hash function to conver the galaxy name to an integer.
  (Variables|Default|SetRandomStream "")
  (for _index (range 0 (- (Utilities|String|Len _galaxyname) 1))
    (LocalVariables|SetSeedInitalValue (Math|Integer|%(Integer) (+ (LocalVariables|GetSeedInitalValue) (* (Utilities|String|GetCharacterasNumber _galaxyname) (Math|Integer|%(Integer) (Math|Float|Truncate (Math|Float|Power (Math|Conversions|ToFloat(Integer) (LocalVariables|GetP)) (Math|Conversions|ToFloat(Integer) _index))) (LocalVariables|GetM)))) (LocalVariables|GetM))))
  (Variables|Default|SetRandomStream (Math|Random|MakeRandomStream (LocalVariables|GetSeedInitalValue))))

(fn GenerateSystemData
  (bind _randomstream (Variables|Default|GetRandomStream))
  (bind _outrownames (DataTable|GetDataTableRowNames "/Game/WorldGeneration/GalaxyMap/DT_StarSystemNames.DT_StarSystemNames"))
  (LocalVariables|SetPossibleSystemNames _outrownames)
  (for _index (range 1 (Variables|Default|GetNumberOfStarSystems))
    (LocalVariables|SetNameIndex (.OutIndex (Utilities|Array|RandomFromStream (LocalVariables|GetPossibleSystemNames) (Variables|Default|GetRandomStream))))
    (while (Utilities|Set|Contains (LocalVariables|GetTakenNames) (Utilities|Array|Get(acopy) (LocalVariables|GetPossibleSystemNames) (LocalVariables|GetNameIndex)))
      (bind _result (Math|Integer|IncrementInt (LocalVariables|GetNameIndex))
        (:%20%20
          (LocalVariables|SetNameIndex (Math|Integer|%(Integer) _result (Utilities|Array|Length (LocalVariables|GetPossibleSystemNames)))))))
    (Utilities|Array|Add (Variables|Default|GetStarSystemData) (Utilities|Struct|MakeS_GalaxyMap_StarSystemData (Utilities|String|ToString(Name) (Utilities|Array|Get(acopy) (LocalVariables|GetPossibleSystemNames) (LocalVariables|GetNameIndex))) (Class|KismetMathLibrary|GetRotated2D (Math|Vector2D|MakeVector2D (Math|Random|RandomFloatinRangefromStream 0.0 (Variables|Default|GetGalaxyRadius) _randomstream) 0.0) (Math|Random|RandomFloatinRangefromStream 0.0 3.6e+02 _randomstream))))
    (Utilities|Set|Add (LocalVariables|GetTakenNames) (Utilities|Array|Get(acopy) (LocalVariables|GetPossibleSystemNames) (LocalVariables|GetNameIndex))))
  (CallFunction|SaveGalaxyMap (Variables|Default|GetStarSystemData) 0.0))

(fn SpawnGalaxyMap
  (for _array_element (Variables|Default|GetStarSystemData)
    (Game|SpawnActorfromClass "/Game/WorldGeneration/GalaxyMap/BP_GalaxyMap_StarSystem.BP_GalaxyMap_StarSystem_C" (Math|Transform|MakeTransform (Math|Conversions|ToVector(Vector2D) (.systeminitallocation _array_element)) "0, 0, 0" "1,1,1") "AdjustIfPossibleButDontSpawnIfColliding" 0 (.systemid _array_element) 0)))