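; Game mode for the galaxy map that shows its HUD and travel arrows, loads or generates the galaxy, then spawns its star system actors.
; Without a save, a random stream seeded by the galaxy name picks unique DataTable names and polar-random positions within the galaxy radius, then saves the result.
; Each system becomes a BP_GalaxyMap_StarSystem on the Z=0 plane, registered by system ID.
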(event EventBeginPlay
  (bind (_galaxyfound _starsystemdata _currentstarsystemid _galaxytime) (CallFunction|LoadGalaxyData))
  (UserInterface|Viewport|AddtoViewport (Variables|/Game/GameInfrastructure/BP_Voidsinger_GameInstance.BP_Voidsinger_GameInstance_C|GetGalaxyMap_HUD (CallFunction|GetVoidsingerGameInstance)) 0)
  (if _galaxyfound
    (bind _values (Utilities|Map|Values _starsystemdata))
    (Variables|Default|SetStarSystemData _values)
    (Variables|Default|SetGalaxy%20Time _galaxytime)
    (else
      (Variables|Default|SetRandomStream (CallFunction|GenerateRandomStreamfromSeed (Variables|/Game/GameInfrastructure/BP_Voidsinger_GameInstance.BP_Voidsinger_GameInstance_C|GetGalaxyName (CallFunction|GetVoidsingerGameInstance))))
      (CallFunction|GenerateSystemData)))
  (CallFunction|SpawnGalaxyMap))

(fn ConstructionScript)

(fn GenerateSystemData
  (bind _randomstream (Variables|Default|GetRandomStream))
  (bind _outrownames (DataTable|GetDataTableRowNames "/Game/WorldGeneration/GalaxyMap/DT_StarSystemNames.DT_StarSystemNames"))
  (LocalVariables|SetPossibleSystemNames _outrownames)
  (for _index (range 1 (Variables|Default|GetNumberOfStarSystems))
    (LocalVariables|SetNameIndex (.OutIndex (Utilities|Array|RandomFromStream (LocalVariables|GetPossibleSystemNames) (Variables|Default|GetRandomStream))))
    (while (Utilities|Set|Contains (LocalVariables|GetTakenNames) (Utilities|Array|Get(acopy) (LocalVariables|GetPossibleSystemNames) (LocalVariables|GetNameIndex)))
      (bind _result (Math|Integer|IncrementInt (LocalVariables|GetNameIndex))
        (:%20%20
          (LocalVariables|SetNameIndex (Math|Integer|%(Integer) _result (Utilities|Array|Length (LocalVariables|GetPossibleSystemNames)))))))
    (Utilities|Map|Add (LocalVariables|GetStarSystemDataToSave) (Utilities|String|ToString(Name) (Utilities|Array|Get(acopy) (LocalVariables|GetPossibleSystemNames) (LocalVariables|GetNameIndex))) (Utilities|Struct|MakeS_GalaxyMap_StarSystemData (Utilities|String|ToString(Name) (Utilities|Array|Get(acopy) (LocalVariables|GetPossibleSystemNames) (LocalVariables|GetNameIndex))) (Utilities|Struct|MakeS_StarSystemTransform (Class|KismetMathLibrary|GetRotated2D (Math|Vector2D|MakeVector2D (Math|Random|RandomFloatinRangefromStream 0.0 (Variables|Default|GetGalaxyRadius) _randomstream) 0.0) (Math|Random|RandomFloatinRangefromStream 0.0 3.6e+02 _randomstream)) (Math|Random|RandomFloatinRangefromStream 0.0 3.6e+02 _randomstream)) (Math|Random|RandomIntegerinRangefromStream 1 10 _randomstream)))
    (Utilities|Set|Add (LocalVariables|GetTakenNames) (Utilities|Array|Get(acopy) (LocalVariables|GetPossibleSystemNames) (LocalVariables|GetNameIndex))))
  ;[1 1 1] Save new galaxy
  (CallFunction|SaveGalaxyData (LocalVariables|GetStarSystemDataToSave) "" 0.0)
  (bind _values (Utilities|Map|Values (LocalVariables|GetStarSystemDataToSave)))
  (Variables|Default|SetStarSystemData _values))

(fn SpawnGalaxyMap
  (for _array_element (Variables|Default|GetStarSystemData)
    (bind _returnvalue (Game|SpawnActorfromClass "/Game/WorldGeneration/GalaxyMap/BP_GalaxyMap_StarSystem.BP_GalaxyMap_StarSystem_C" (Math|Transform|MakeTransform (Math|Conversions|ToVector(Vector2D) (.loaction (.systeminitallocation _array_element))) (Math|Rotator|MakeRotator 0.0 0.0 (.rotation (.systeminitallocation _array_element))) "1,1,1") "AdjustIfPossibleButDontSpawnIfColliding" 0 (.systemid _array_element) 0))
    (Utilities|Map|Add (Variables|Default|GetSystemActors) (.systemid _array_element) _returnvalue)))