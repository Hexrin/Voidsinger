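; Procedural galaxy actor that loads a saved star map on BeginPlay, or generates and saves a new one.
; GenerateSeed applies a polynomial hash to the galaxy name, though it reads only the first character on every iteration.
; GenerateSystemData picks unique DataTable names through seeded streams, probing past taken ones, but places systems at unseeded random polar positions within the galaxy radius.
; SpawnGalaxyMap is an empty stub.
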(event EventBeginPlay
  (bind (_galaxyfound _systemdata _galaxytime) (CallFunction|LoadGalaxyMap))
  (if _galaxyfound
    (Variables|Default|SetSystemData _systemdata)
    (Variables|Default|SetGalaxy%20Time _galaxytime)
    (else
      (CallFunction|GenerateSeed)
      (CallFunction|GenerateSystemData))))

(fn ConstructionScript)

(fn GenerateSeed
  (bind _asbp_void_game_instance (CallFunction|GetVoidGameInstance))
  (bind _galaxyname (Variables|/Game/GameInfrastructure/BP_VoidGameInstance.BP_VoidGameInstance_C|GetGalaxyName _asbp_void_game_instance))
  ;[0 0 1] Uses a polynomial rolling hash function to conver the galaxy name to an integer.
  (Variables|Default|SetSeed 0)
  (for _index (range 0 (- (Utilities|String|Len _galaxyname) 1))
    (Variables|Default|SetSeed (Math|Integer|%(Integer) (+ (Variables|Default|GetSeed) (* (Utilities|String|GetCharacterasNumber _galaxyname) (Math|Integer|%(Integer) (Math|Float|Truncate (Math|Float|Power (Math|Conversions|ToFloat(Integer) (LocalVariables|GetP)) (Math|Conversions|ToFloat(Integer) _index))) (LocalVariables|GetM)))) (LocalVariables|GetM)))))

(fn GenerateSystemData
  (bind _outrownames (DataTable|GetDataTableRowNames "/Game/WorldGeneration/GalaxyMap/DT_StarSystemNames.DT_StarSystemNames"))
  (LocalVariables|SetPossibleSystemNames _outrownames)
  (for _index (range 1 (Variables|Default|GetNumberOfStarSystems))
    (LocalVariables|SetNameIndex (.OutIndex (Utilities|Array|RandomFromStream (LocalVariables|GetPossibleSystemNames) (Math|Random|MakeRandomStream (+ (Variables|Default|GetSeed) _index)))))
    (while (Utilities|Set|Contains (LocalVariables|GetTakenNames) (Utilities|Array|Get(acopy) (LocalVariables|GetPossibleSystemNames) (LocalVariables|GetNameIndex)))
      (bind _result (Math|Integer|IncrementInt (LocalVariables|GetNameIndex))
        (:%20%20
          (LocalVariables|SetNameIndex (Math|Integer|%(Integer) _result (Utilities|Array|Length (LocalVariables|GetPossibleSystemNames)))))))
    (Utilities|Array|Add (Variables|Default|GetStarSystemData) (Utilities|Struct|MakeS_GalaxyMapStarSystemData (Utilities|String|ToString(Name) (Utilities|Array|Get(acopy) (LocalVariables|GetPossibleSystemNames) (LocalVariables|GetNameIndex))) (Class|KismetMathLibrary|GetRotated2D (Math|Vector2D|MakeVector2D (Math|Random|RandomFloatinRange 0.0 (Variables|Default|GetGalaxyRadius)) 0.0) (Math|Random|RandomFloatinRange 0.0 3.6e+02))))
    (Utilities|Set|Add (LocalVariables|GetTakenNames) (Utilities|Array|Get(acopy) (LocalVariables|GetPossibleSystemNames) (LocalVariables|GetNameIndex))))
  (CallFunction|SaveGalaxyMap (Variables|Default|GetStarSystemData) 0.0))

(fn SpawnGalaxyMap)