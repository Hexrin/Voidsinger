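; Star system actor for the galaxy map, with a main star, a highlight widget and surrounding decorative stars.
; The construction script sizes a collision sphere to the widget to prevent overlap and tints the main star from cyan to red, brightening it by system tier.
; It scatters seeded random star meshes, keyed on galaxy name and current system ID rather than its own SystemID.
; BeginPlay hands the actor reference to the highlight widget.
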(event EventBeginPlay
  (Variables|/Game/UI/WorldGeneration/GalaxyMap/WBP_GalaxyMap_StarSystemHighlight.WBP_GalaxyMap_StarSystemHighlight_C|SetSystemRef (.AsWBP%20Galaxy%20Map%20Star%20System%20Highlight (Utilities|Casting|CastToWBP_GalaxyMap_StarSystemHighlight (UserInterface|GetWidget (Variables|Default|GetWidget)))) self))

(fn ConstructionScript
  (bind _starsystemdata (CallFunction|LoadGalaxyData))
  (bind _returnvalue (Class|KismetSystemLibrary|MakeLiteralInteger 10))
  (bind _systemid (Variables|Default|GetSystemID))
  (bind _value (Utilities|Map|Find _starsystemdata _systemid))
  (bind _returnvalue_2 (- _returnvalue 1))
  (bind _returnvalue_3 (- (.systemtier _value) 1))
  (bind _returnvalue_4 (/ _returnvalue_3 _returnvalue_2))
  ;[1 1 1] Add sphere collision to prevent star system overlap
  (Components|Sphere|SetSphereRadius (Variables|Default|GetSphere) (.SphereRadius (Collision|GetComponentBounds (Variables|Default|GetWidget))) true)
  ;[1 1 1] Update main star material to match difficulty
  (bind _returnvalue_5 (Rendering|Material|CreateDynamicMaterialInstance (Variables|Default|GetMainStar) 0 "/Game/2DAssets/WorldGeneration/GalaxyMap/M_Star.M_Star" "None" :!class /Script/Engine.PrimitiveComponent))
  (Rendering|Material|SetVectorParameterValue _returnvalue_5 "Color" (Class|KismetMathLibrary|LinearColorLerpUsingHSV "(R=0.000000,G=1.000000,B=0.916667,A=1.000000)" "(R=1.000000,G=0.000000,B=0.000000,A=1.000000)" _returnvalue_4) :!class /Script/Engine.MaterialInstanceDynamic)
  (Rendering|Material|SetScalarParameterValue _returnvalue_5 "Brightness" (Math|Float|Lerp 1e+01 5e+01 _returnvalue_4) :!class /Script/Engine.MaterialInstanceDynamic)
  ;[1 1 1] Generate Backround Stars
  (LocalVariables|SetRandomStream (CallFunction|GenerateRandomStreamfromSeed (Utilities|String|Append (Variables|/Game/GameInfrastructure/BP_Voidsinger_GameInstance.BP_Voidsinger_GameInstance_C|GetGalaxyName (CallFunction|GetVoidsingerGameInstance)) (.CurrentStarSystemID (CallFunction|LoadGalaxyData)))))
  (for _index (range 0 (Class|KismetMathLibrary|RandomIntegerfromStream 500 (LocalVariables|GetRandomStream)))
    (bind _returnvalue_6 (AddComponent|AddStaticMeshComponent false (Math|Transform|MakeTransform (* (Math|Random|RandomUnitVectorinConeinDegreesfromStream (Math|Vector|MakeVector 0.0 0.0 -1.0) 8e+01 (LocalVariables|GetRandomStream)) (Math|Random|RandomFloatinRangefromStream 0.5 1e+01 (LocalVariables|GetRandomStream))) (Math|Rotator|MakeRotator 0.0 0.0 (Math|Random|RandomFloatinRangefromStream 0.0 3.6e+02 (LocalVariables|GetRandomStream))) (Math|Conversions|ToVector(Float) (Math|Random|RandomFloatinRangefromStream 0.05 0.3 (LocalVariables|GetRandomStream))))))
    (bind _returnvalue_7 (Rendering|Material|CreateDynamicMaterialInstance _returnvalue_6 0 "/Game/2DAssets/WorldGeneration/GalaxyMap/M_Star.M_Star" "None" :!class /Script/Engine.PrimitiveComponent))
    (Rendering|Material|SetVectorParameterValue _returnvalue_7 "Color" (Class|KismetMathLibrary|HSVtoRGB (Math|Random|RandomFloatinRangefromStream 0.0 3.6e+02 (LocalVariables|GetRandomStream)) (Math|Random|RandomFloatinRangefromStream 0.5 1.0 (LocalVariables|GetRandomStream)) 1.0 1.0) :!class /Script/Engine.MaterialInstanceDynamic)
    (Rendering|Material|SetScalarParameterValue _returnvalue_7 "Brightness" (Math|Random|RandomFloatinRangefromStream 2.0 1e+01 (LocalVariables|GetRandomStream)) :!class /Script/Engine.MaterialInstanceDynamic)))