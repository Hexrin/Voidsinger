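; Star system actor that populates the current system with enemy ships and opens the galaxy map when the player leaves its zone.
; On BeginPlay it restores saved actors, or generates groups from a seeded stream, splitting system difficulty by group spawn mode across demo enemy classes.
; SystemZone overlaps track which ships belong, and their classes and transforms are saved on EndPlay or destruction.
; The construction script sizes both zones and the background from radius settings.
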(event OnComponentEndOverlap(SystemZone)
  (params (OverlappedComponent :type Primitive%20Component%20Object%20Reference) (OtherActor :type Actor%20Object%20Reference) (OtherComp :type Primitive%20Component%20Object%20Reference) (OtherBodyIndex :type Integer))
  (if (== OtherActor (Game|Player|GetPlayerPawn 0))
    (CallFunction|OpenGalaxyMap)
    (else
      (bind _asbp_base_enemy_ship (Utilities|Casting|CastToBP_BaseEnemyShip OtherActor))
      (CallFunction|PreventStarSystemActorRespawn _asbp_base_enemy_ship))))

(event OnComponentBeginOverlap(SystemZone)
  (params (OverlappedComponent :type Primitive%20Component%20Object%20Reference) (OtherActor :type Actor%20Object%20Reference) (OtherComp :type Primitive%20Component%20Object%20Reference) (OtherBodyIndex :type Integer) (bFromSweep :type Boolean) (SweepResult :type Hit%20Result%20Structure%20%28by%20ref%29))
  (bind _asbp_base_enemy_ship (Utilities|Casting|CastToBP_BaseEnemyShip OtherActor))
  (Utilities|Array|AddUnique (Variables|Private|GetSpawned%20Actors) _asbp_base_enemy_ship))

(event EventBeginPlay
  (bind _currentstarsystemid (CallFunction|LoadGalaxyMap))
  (bind (_galaxyfound _starsystemdata _currentstarsystemid_2 _galaxytime) (CallFunction|LoadGalaxyMap))
  (bind (_system_found _actordata) (CallFunction|LoadStarSystem _currentstarsystemid))
  ;[0 1 0] Determine if the player has already visited this star system.
  (if _system_found
    ;[1 1 1] Load Existing Star System
    (for _array_element _actordata
      (if (< (Math|Vector|VectorLengthSquared (.Location (Math|Transform|BreakTransform (.transform _array_element)))) (Math|Vector|VectorLengthSquared (Variables|Default|GetSystemRadius)))
        (bind _returnvalue (Game|SpawnActorfromClass (.class _array_element) (.transform _array_element) "AlwaysSpawn" 0 0))
        (Utilities|Array|Add (Variables|Private|GetSpawned%20Actors) _returnvalue)))
    (else
      ;[1 1 1] Generate New Star System
      (Variables|Private|SetRandomStream (CallFunction|GenerateRandomStreamfromSeed (Utilities|String|Append (Variables|/Game/GameInfrastructure/BP_Voidsinger_GameInstance.BP_Voidsinger_GameInstance_C|GetGalaxyName (CallFunction|GetVoidsingerGameInstance)) _currentstarsystemid_2 (Utilities|String|ToString(Float) _galaxytime))))
      (for _index (range 0 (Math|Random|RandomIntegerinRangefromStream (Variables|ShipSpawnSettings|GetMinShipGroupsToSpawn) (Variables|ShipSpawnSettings|GetMaxShipGroupsToSpawn) (Variables|Private|GetRandomStream)))
        (ShipSpawning|SpawnEnemyGroup (.systemdifficulty (CallFunction|GetStarSystemData)))))))

(event EventEndPlay
  (params (EndPlayReason :type EEndPlayReason%20Enum :default "Destroyed"))
  (CallFunction|SaveStarSystemData))

(event EventDestroyed
  (CallFunction|SaveStarSystemData))

(fn ConstructionScript
  (bind _enemy_spawn_zone (Variables|Default|GetEnemy%20Spawn%20Zone))
  (bind _levelbackground (Variables|Default|GetLevelBackground))
  (bind _returnvalue (Components|Sphere|GetScaledSphereRadius _enemy_spawn_zone))
  (bind _output_get (Variables|ShipSpawnSettings|SetSpawnRadius (Math|Conversions|ToVector(Vector2D) (Math|Conversions|ToVector2D(Vector) (Variables|ShipSpawnSettings|GetSpawnRadius)))))
  (Components|Sphere|SetSphereRadius (Variables|Default|GetEnemy%20Spawn%20Zone) (Math|Vector|VectorLengthXY _output_get) true)
  (bind _output_get_2 (Variables|Default|SetSystemRadius (Math|Conversions|ToVector(Vector2D) (Math|Conversions|ToVector2D(Vector) (Math|Vector|VectorClampSize2D (Variables|Default|GetSystemRadius) (Class|SphereComponent|GetUnscaledSphereRadius (Variables|Default|GetEnemy%20Spawn%20Zone)) 99999997952.0)))))
  (Components|Sphere|SetSphereRadius (Variables|Default|GetSystem%20Zone) (Math|Vector|VectorLengthXY _output_get_2) true)
  (Niagara|SetNiagaraVariable(Float) _levelbackground "Radius" _returnvalue)
  (Niagara|SetNiagaraVariable(Float) _levelbackground "TorrusHandelRadius" (- (Components|Sphere|GetScaledSphereRadius (Variables|Default|GetSystem%20Zone)) _returnvalue)))

(fn SpawnEnemyGroup
  (params (Group%20Difficulty :type Integer))
  (bind _randomstream (Variables|Private|GetRandomStream))
  (LocalVariables|SetSpawnPoints Group%20Difficulty)
  (Development|PrintString "Spawn Group" true true "(R=0.000000,G=0.660000,B=1.000000,A=1.000000)" 1e+03)
  ;[0 0 1] Gets a random inital spawn diffiuculty
  (LocalVariables|SetDifficultyToSpawn (ShipSpawning|RandomDifficulty (- Group%20Difficulty (- (Variables|ShipSpawnSettings|GroupSettings|GetMinShipGroupSize) 1))))
  ;[0 0 1] Get random location inside Enemy Spawn Zone
  (LocalVariables|SetGroupLocation (* (Class|KismetMathLibrary|RandomUnitVectorinEllipticalConeinDegreesfromStream (Math|Vector|MakeVector 1.0 0.0 0.0) 3.6e+02 0.0 _randomstream) (Math|Random|RandomFloatinRangefromStream 0.0 (Components|Sphere|GetScaledSphereRadius (Variables|Default|GetEnemy%20Spawn%20Zone)) _randomstream)))
  ;[1 1 1] Spawn new ships until the difficult quota has been met
  (while (> (LocalVariables|GetSpawnPoints) 0)
    (switch Utilities|FlowControl|Switch|SwitchonE_EnemySpawnMode (Variables|ShipSpawnSettings|GroupSettings|GetGroupSpawnMode)
      (:NewEnumerator0
        ;;[1 1 1] Spawns enemies of the same class until the spawn quota has been met
        (if (Utilities|IsValidClass (LocalVariables|GetClassToSpawn))
          _
          (else
            (LocalVariables|SetClassToSpawn (.OutItem (Utilities|Array|RandomFromStream (ShipSpawning|GetEnemyClassesOfDifficultyRating (LocalVariables|GetDifficultyToSpawn)) (Variables|Private|GetRandomStream))))))
        (ShipSpawning|SpawnEnemy (LocalVariables|GetClassToSpawn) (LocalVariables|GetGroupLocation) (Variables|ShipSpawnSettings|GroupSettings|GetGroupSpawnRadius)))
      (:NewEnumerator1
        ;;[1 1 1] Spawns enemies of the same difficulty until the spawn quota has been met
        (ShipSpawning|SpawnEnemy (.OutItem (Utilities|Array|RandomFromStream (ShipSpawning|GetEnemyClassesOfDifficultyRating (LocalVariables|GetDifficultyToSpawn)) (Variables|Private|GetRandomStream))) (LocalVariables|GetGroupLocation) (Variables|ShipSpawnSettings|GroupSettings|GetGroupSpawnRadius)))
      (:NewEnumerator2
        ;;[1 1 1] Spawns enemies of a random difficulty until the spawn quota has been met
        (LocalVariables|SetDifficultyToSpawn (select (>= (+ (LocalVariables|GetShipsSpawned) 2) (Variables|ShipSpawnSettings|GroupSettings|GetMaxShipGroupSize)) (LocalVariables|GetSpawnPoints) (ShipSpawning|RandomDifficulty (LocalVariables|GetSpawnPoints))))
        (ShipSpawning|SpawnEnemy (.OutItem (Utilities|Array|RandomFromStream (ShipSpawning|GetEnemyClassesOfDifficultyRating (LocalVariables|GetDifficultyToSpawn)) (Variables|Private|GetRandomStream))) (LocalVariables|GetGroupLocation) (Variables|ShipSpawnSettings|GroupSettings|GetGroupSpawnRadius))))
    (LocalVariables|SetSpawnPoints (- (LocalVariables|GetSpawnPoints) (LocalVariables|GetDifficultyToSpawn)))
    (Math|Integer|IncrementInt (LocalVariables|GetShipsSpawned))))

(fn GetEnemyClassesOfDifficultyRating
  (params (Rating :type Integer))
  (for _array_element (CallFunction|GetChildClasses "/Game/Ships/BP_BaseEnemyShip.BP_BaseEnemyShip_C")
    (if (and (Utilities|String|Contains (Utilities|GetClassDisplayName (.AsBP%20Base%20Enemy%20Ship (Utilities|Casting|CastToBP_BaseEnemyShipClass _array_element))) "demo") (== (Utilities|GetClassDefaults (.AsBP%20Base%20Enemy%20Ship (Utilities|Casting|CastToBP_BaseEnemyShipClass _array_element))) Rating))
      (Utilities|Array|Add (LocalVariables|GetReturnValue) (.AsBP%20Base%20Enemy%20Ship (Utilities|Casting|CastToBP_BaseEnemyShipClass _array_element)))))
  (return (LocalVariables|GetReturnValue)))

(fn SpawnEnemy
  (params (Class :type BP%20Base%20Enemy%20Ship%20Class%20Reference) (Location :type Vector) (GroupSpawnRadius :type Float%20%28single-precision%29))
  (Development|PrintString (Utilities|String|Append "Spawn Enemy of Diffiuculty " (Utilities|String|ToString(Integer) (Utilities|GetClassDefaults Class))) true true "(R=0.000000,G=0.260104,B=0.394097,A=1.000000)" 1e+03)
  (bind _returnvalue (Game|SpawnActorfromClass Class (Math|Transform|MakeTransform (+ Location (Math|Vector|RotateVector (Math|Vector|MakeVector GroupSpawnRadius 0.0 0.0) (Math|Rotator|MakeRotator 0.0 0.0 (Math|Random|RandomFloatinRange 0.0 3.6e+02)))) (Math|Rotator|MakeRotator 0.0 0.0 (Math|Random|RandomFloatinRange 0.0 3.6e+02)) "1,1,1") "AdjustIfPossibleButAlwaysSpawn" 0 0))
  (Utilities|Array|Add (Variables|Private|GetSpawned%20Actors) _returnvalue))

(fn RandomDifficulty
  (params (SpawnPoints :type Integer))
  ;[0 0 1] Gets a random diffiuclty that won't result in spawing more or less ships than Ship Group Size will allow
  (for _index (range 1 SpawnPoints)
    (if (Utilities|Select :Index (Variables|ShipSpawnSettings|GroupSettings|GetGroupSpawnMode) :NewEnumerator0 (and (== (Math|Integer|%(Integer) SpawnPoints _index) 0) (Math|Integer|InRange(Integer) (/ SpawnPoints _index) (Variables|ShipSpawnSettings|GroupSettings|GetMinShipGroupSize) (Variables|ShipSpawnSettings|GroupSettings|GetMaxShipGroupSize))) :NewEnumerator1 (and (== (Math|Integer|%(Integer) SpawnPoints _index) 0) (Math|Integer|InRange(Integer) (/ SpawnPoints _index) (Variables|ShipSpawnSettings|GroupSettings|GetMinShipGroupSize) (Variables|ShipSpawnSettings|GroupSettings|GetMaxShipGroupSize))) :NewEnumerator2 true)
      (Utilities|Array|Add (LocalVariables|GetPossibe%20Spawns) _index)))
  (return (.OutItem (Utilities|Array|RandomFromStream (LocalVariables|GetPossibe%20Spawns) (Variables|Private|GetRandomStream)))))

(fn SaveStarSystemData
  (for _array_element (Variables|Private|GetSpawned%20Actors)
    (Utilities|IsValid _array_element
      (:Is%20Valid
        (Utilities|Array|Add (LocalVariables|GetActorData) (Utilities|Struct|MakeS_StarSystemActorData (Utilities|GetClass _array_element) (Transformation|GetActorTransform _array_element))))))
  (CallFunction|SaveStarSystem (.CurrentStarSystemID (CallFunction|LoadGalaxyMap)) (LocalVariables|GetActorData)))

(fn PreventStarSystemActorRespawn
  (params (Actor :type Actor%20Object%20Reference))
  (Utilities|Array|RemoveItem (Variables|Private|GetSpawned%20Actors) Actor))