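; Level manager for a star system map that spawns the player ship and the star system and handles player death.
; On BeginPlay it spawns the ship at a fixed offset, spawns and stores a BP_StarSystem configured for ship groups and radius, then notifies the game instance that the system opened.
; The construction script binds the player death event, which adds the death screen widget to the viewport.
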(event EventBeginPlay
  (Game|SpawnActorfromClass "/Game/Ships/BP_PlayerShip.BP_PlayerShip_C" (Math|Transform|MakeTransform "-1250.000000, 0, 0" "0, 0, 0" "1,1,1") "Undefined" self 0)
  (bind _returnvalue (Game|SpawnActorfromClass "/Game/WorldGeneration/StarSystem/BP_StarSystem.BP_StarSystem_C" (Math|Transform|MakeTransform "0, 0, 0" "0, 0, 0" "1,1,1") "Undefined" self 1 3 "NewEnumerator2" 3 1 2.5e+02 1.5e+03 2.25e+03 0))
  (Variables|Default|SetStarSystemRef _returnvalue)
  (Default|CallOnStarSystemOpened (CallFunction|GetVoidsingerGameInstance)))

(fn ConstructionScript
  (EventDispatchers|BindEventtoOnPlayerDeath (EventDispatchers|CreateEvent :!event PlayerDeath)))

(fn PlayerDeath
  (bind _returnvalue (UserInterface|CreateWidget "/Game/UI/PlayerDeath/UMG_PlayerDeath.UMG_PlayerDeath_C"))
  (UserInterface|Viewport|AddtoViewport _returnvalue 0))