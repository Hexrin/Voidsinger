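; Game mode for a star system level that builds the system and places the player in it on BeginPlay.
; It spawns BP_StarSystem with its ship group and radius settings, spawns the player ship on negative X at the spawn radius's length, then notifies the Voidsinger game instance that the system opened.
; The construction script binds to the player death event, and PlayerDeath adds the death widget to the viewport.
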(event EventBeginPlay
  (bind _returnvalue (Game|SpawnActorfromClass "/Game/WorldGeneration/StarSystem/BP_StarSystem.BP_StarSystem_C" (Math|Transform|MakeTransform "0, 0, 0" "0, 0, 0" "1,1,1") "Undefined" 0 (Variables|Default|GetMin%20Ship%20Groups%20to%20Spawn) (Variables|Default|GetMax%20Ship%20Groups%20to%20Spawn) (Variables|Default|GetGroup%20Spawn%20Mode) (Variables|Default|GetMax%20Ship%20Group%20Size) (Variables|Default|GetMin%20Ship%20Group%20Size) (Variables|Default|GetGroup%20Spawn%20Radius) (Variables|Default|GetSpawn%20Radius) (Variables|Default|GetSystem%20Radius) 0))
  (Variables|Default|SetStarSystemRef _returnvalue)
  (Game|SpawnActorfromClass "/Game/Ships/BP_PlayerShip.BP_PlayerShip_C" (Math|Transform|MakeTransform (Math|Vector|MakeVector (* (Math|Vector|VectorLength (Variables|Default|GetSpawn%20Radius)) -1.0) 0.0 0.0) "0, 0, 0" "1,1,1") "Undefined" 0 0)
  (Default|CallOnStarSystemOpened (CallFunction|GetVoidsingerGameInstance)))

(fn ConstructionScript
  (EventDispatchers|BindEventtoOnPlayerDeath (EventDispatchers|CreateEvent :!event PlayerDeath)))

(fn PlayerDeath
  (bind _returnvalue (UserInterface|CreateWidget "/Game/UI/PlayerDeath/UMG_PlayerDeath.UMG_PlayerDeath_C"))
  (UserInterface|Viewport|AddtoViewport _returnvalue 0))