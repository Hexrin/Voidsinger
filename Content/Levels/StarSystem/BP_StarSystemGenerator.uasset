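; Star system generator that populates a level with a random number of enemy ship groups at BeginPlay.
; The construction script sizes a flat spawn box, inside which each group gets a random center.
; Each group spends a difficulty budget on game-instance enemy classes matching a randomly rolled rating, with GroupSpawnMode steering selection.
; Ships spawn with random yaw at random angles on a fixed-radius ring around that center.
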(event EventBeginPlay
  (for _index (range 0 (Math|Random|RandomIntegerinRange (Variables|Default|GetMinShipGroupsToSpawn) (Variables|Default|GetMaxShipGroupsToSpawn)))
    (CallFunction|SpawnEnemyGroup (Variables|Default|GetDifficulty%20Rating))))

(fn ConstructionScript
  (bind _output_get (Variables|Default|SetSpawnExtent (Math|Conversions|ToVector(Vector2D) (Math|Conversions|ToVector2D(Vector) (Variables|Default|GetSpawnExtent)))))
  (Components|Box|SetBoxExtent (Variables|Default|GetEnemy%20Spawn%20Zone) (Math|Vector|VectorGetAbs _output_get) true))

(fn SpawnEnemyGroup
  (params (Group%20Difficulty :type Integer))
  (bind _enemy_spawn_zone (Variables|Default|GetEnemy%20Spawn%20Zone))
  (LocalVariables|SetSpawnPoints Group%20Difficulty)
  (LocalVariables|SetDifficultyToSpawn (CallFunction|RandomDifficulty Group%20Difficulty))
  ;[0 0 1] Get random location inside Enemy Spawn Zone
  (LocalVariables|SetGroupLocation (+ (Math|Vector|RotateVector (Math|Random|RandomPointinBoundingBox "0, 0, 0" (Components|Box|GetScaledBoxExtent _enemy_spawn_zone)) (Transformation|GetWorldRotation _enemy_spawn_zone)) (Transformation|GetWorldLocation _enemy_spawn_zone)))
  (while (> (LocalVariables|GetSpawnPoints) 0)
    (switch Utilities|FlowControl|Switch|SwitchonE_EnemySpawnMode (Variables|Default|GetGroupSpawnMode)
      (:NewEnumerator0
        (if (Utilities|IsValidClass (LocalVariables|GetClassToSpawn))
          _
          (else
            (LocalVariables|SetClassToSpawn (.OutItem (Utilities|Array|Random (CallFunction|GetEnemyClassesOfDifficultyRating (LocalVariables|GetDifficultyToSpawn)))))))
        (CallFunction|SpawnEnemy (LocalVariables|GetClassToSpawn) (LocalVariables|GetGroupLocation) (Variables|Default|GetGroupSpawnRadius)))
      (:NewEnumerator1
        (CallFunction|SpawnEnemy (.OutItem (Utilities|Array|Random (CallFunction|GetEnemyClassesOfDifficultyRating (LocalVariables|GetDifficultyToSpawn)))) (LocalVariables|GetGroupLocation) (Variables|Default|GetGroupSpawnRadius)))
      (:NewEnumerator2
        (LocalVariables|SetSpawnPoints (CallFunction|RandomDifficulty (LocalVariables|GetSpawnPoints)))
        (CallFunction|SpawnEnemy (.OutItem (Utilities|Array|Random (CallFunction|GetEnemyClassesOfDifficultyRating (LocalVariables|GetDifficultyToSpawn)))) (LocalVariables|GetGroupLocation) (Variables|Default|GetGroupSpawnRadius))))
    (LocalVariables|SetSpawnPoints (- (LocalVariables|GetSpawnPoints) (LocalVariables|GetDifficultyToSpawn)))))

(fn GetEnemyClassesOfDifficultyRating
  (params (Rating :type Integer))
  (for _array_element (Variables|/Game/GameInfrastructure/BP_VoidGameInstance.BP_VoidGameInstance_C|GetEnemyClasses (CallFunction|GetVoidGameInstance))
    (if (== (Utilities|GetClassDefaults _array_element) Rating)
      (Utilities|Array|Add (LocalVariables|GetReturnValue) _array_element)))
  (return (LocalVariables|GetReturnValue)))

(fn SpawnEnemy
  (params (Class :type BP%20Base%20Enemy%20Ship%20Class%20Reference) (Location :type Vector) (GroupSpawnRadius :type Float%20%28single-precision%29))
  (Game|SpawnActorfromClass Class (Math|Transform|MakeTransform (+ Location (Math|Vector|RotateVector (Math|Vector|MakeVector GroupSpawnRadius 0.0 0.0) (Math|Rotator|MakeRotator 0.0 0.0 (Math|Random|RandomFloatinRange 0.0 3.6e+02)))) (Math|Rotator|MakeRotator 0.0 0.0 (Math|Random|RandomFloatinRange 0.0 3.6e+02)) "1,1,1") "Undefined" 0 0))

(fn RandomDifficulty
  (params (MaxDifficulty :type Integer))
  (return (Math|Random|RandomIntegerinRange (Math|Integer|Max(Integer) (+ (- MaxDifficulty (Variables|Default|GetMaxShipGroupSize)) 1) 1) MaxDifficulty)))