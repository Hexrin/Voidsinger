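; BP_Voidsong_Verb_Disperse is the Voidsong verb that shoves a hit ship away from where the song was called.
; On Activate it casts the hit actor to BaseShip and applies a 2D impulse to that ship's PhysicsComponent.
; The impulse points from the call location toward the hit location, scaled by effectiveness and DisperseForce.
; It lands at the hit location relative to the ship's position, rather than at its origin.
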(event EventActivate
  (params (NewActorHit :type Actor%20Object%20Reference) (NewActorThatActivated :type Actor%20Object%20Reference) (NewPartsHit :type Array%20of%20Base%20Part%20Object%20References) (NewLocationCalledFrom :type Vector :default "0, 0, 0") (NewWorldLocation :type Vector :default "0, 0, 0") (NewEffectiveness :type Float%20%28single-precision%29))
  (bind _asbase_ship (Utilities|Casting|CastToBaseShip NewActorHit))
  ;[1 1 1] GET AWAY FROM ME PEASANT
  (Class|ShipPhysicsComponent|AddImpulse (Variables|/Script/Voidsinger.BaseShip|GetPhysicsComponent _asbase_ship) (Math|Conversions|ToVector2D(Vector) (* (Math|Vector|GetUnitDirection(Vector) NewLocationCalledFrom NewWorldLocation) (* NewEffectiveness (Variables|Default|GetDisperseForce)))) (Math|Conversions|ToVector2D(Vector) (- NewWorldLocation (Transformation|GetActorLocation _asbase_ship)))))