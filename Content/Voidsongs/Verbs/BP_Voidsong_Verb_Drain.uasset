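; Voidsong verb that steals resources from the ship parts it hits and gives them to the activating ship.
; On Activate, it drains each system on those parts by DrainAmount scaled by effectiveness, capped at what that system holds.
; It rerolls random resource systems on the activator until the type matches, with no exit if none does.
; The credited amount is recalculated from the target's post-drain level, so can differ from the amount drawn.
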(event EventActivate
  (params (NewActorHit :type Actor%20Object%20Reference) (NewActorThatActivated :type Actor%20Object%20Reference) (NewPartsHit :type Array%20of%20Base%20Part%20Object%20References) (NewLocationCalledFrom :type Vector :default "0, 0, 0") (NewWorldLocation :type Vector :default "0, 0, 0") (NewEffectiveness :type Float%20%28single-precision%29))
  (bind _drainamount (Variables|Default|GetDrainAmount))
  (bind _returnvalue (* NewEffectiveness _drainamount))
  ;[1 1 1] I steal ur stuff heheheheehehehe
  (for _array_element NewPartsHit
    (Utilities|IsValid _array_element
      (:Is%20Valid
        (for _array_element_2 (Class|BasePart|GetSystems _array_element)
          (Class|BaseResourceSystem|DrawResources _array_element_2 (Math|Float|SelectFloat (Class|BaseResourceSystem|GetResourceAmount _array_element_2) _returnvalue (> _returnvalue (Class|BaseResourceSystem|GetResourceAmount _array_element_2))))
          (Utilities|IsValid (Variables|Default|GetRandomSystem)
            (:Is%20Valid
              (while (not (Utilities|Enum|Equal(Enum) (Class|BaseResourceSystem|GetType (Variables|Default|GetRandomSystem)) (Class|BaseResourceSystem|GetType _array_element_2))) :!label _label
                (Variables|Default|SetRandomSystem (.OutItem (Utilities|Array|Random (Class|BaseShip|GetResourceSystems (.AsBase%20Ship (Utilities|Casting|CastToBaseShip NewActorThatActivated)))))))
              (Class|BaseResourceSystem|AddResources (Variables|Default|GetRandomSystem) (Math|Float|SelectFloat (Class|BaseResourceSystem|GetResourceAmount _array_element_2) _returnvalue (> _returnvalue (Class|BaseResourceSystem|GetResourceAmount _array_element_2)))))
            (:Is%20Not%20Valid
              (Utilities|FlowControl|Sequence
                (:then_0
                  (Variables|Default|SetRandomSystem (.OutItem (Utilities|Array|Random (Class|BaseShip|GetResourceSystems (.AsBase%20Ship (Utilities|Casting|CastToBaseShip NewActorThatActivated)))))))
                (:then_1
                  (goto _label))))))))))