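; Voidsong verb that fills systems on the hit ship parts with resources drawn from the activating ship.
; On Activate, it loops through every system of each hit part and repeatedly picks a random resource system on the activator until the types match, with no exit otherwise.
; It then draws and adds FillAmount scaled by effectiveness, capped by the source's current amount, which is re-read after the draw.
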(event EventActivate
  (params (NewActorHit :type Actor%20Object%20Reference) (NewActorThatActivated :type Actor%20Object%20Reference) (NewPartsHit :type Array%20of%20Base%20Part%20Object%20References) (NewLocationCalledFrom :type Vector :default "0, 0, 0") (NewWorldLocation :type Vector :default "0, 0, 0") (NewEffectiveness :type Float%20%28single-precision%29))
  (bind _fillamount (Variables|Default|GetFillAmount))
  (bind _returnvalue (* NewEffectiveness _fillamount))
  ;[1 1 1] Here are some things
  (for _array_element NewPartsHit
    (for _array_element_2 (Class|BasePart|GetSystems _array_element)
      (bind _output_get (Variables|Default|SetRandomSystem (.OutItem (Utilities|Array|Random (Class|BaseShip|GetResourceSystems (.AsBase%20Ship (Utilities|Casting|CastToBaseShip NewActorThatActivated))))) :!label _label))
      (if (Utilities|Enum|Equal(Enum) (Class|BaseResourceSystem|GetType _output_get) (Class|BaseResourceSystem|GetType _array_element_2))
        (Class|BaseResourceSystem|DrawResources _output_get (Math|Float|SelectFloat (Class|BaseResourceSystem|GetResourceAmount _output_get) _returnvalue (> _returnvalue (Class|BaseResourceSystem|GetResourceAmount _output_get))))
        (Class|BaseResourceSystem|AddResources _array_element_2 (Math|Float|SelectFloat (Class|BaseResourceSystem|GetResourceAmount _output_get) _returnvalue (> _returnvalue (Class|BaseResourceSystem|GetResourceAmount _output_get))))
        (else
          (goto _label))))))