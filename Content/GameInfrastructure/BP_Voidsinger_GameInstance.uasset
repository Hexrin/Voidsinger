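; Game instance for Voidsinger that creates the persistent UI widgets and handles transitions between the galaxy map and star systems.
; Init builds the child class map, creates loading, HUD, travel arrow and build widgets, restores Pixels from galaxy data, then opens the galaxy map.
; Transitions show the loading screen and save galaxy or ship state before opening levels, passing SystemID as a URL option.
; GenerateGalaxy loads the named save slot and resets Pixels.
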(event Custom|OpenStarSystem
  (params (StarSystemID :type String))
  (bind _galaxysavestate (Variables|Default|GetGalaxySaveState))
  (Utilities|ActivateLoadingScreen)
  (CallFunction|SaveGalaxyData (Variables|/Game/WorldGeneration/GalaxyMap/BP_GalaxyMap_SaveData.BP_GalaxyMap_SaveData_C|GetStarSystemData _galaxysavestate) StarSystemID (Variables|/Game/WorldGeneration/GalaxyMap/BP_GalaxyMap_SaveData.BP_GalaxyMap_SaveData_C|GetGalaxyTime _galaxysavestate))
  (Utilities|FlowControl|Delay 0.2)
  (Game|OpenLevel(byObjectReference) "/Game/WorldGeneration/StarSystem/LVL_StarSystem.LVL_StarSystem" true (Utilities|String|Append "?SystemID=" StarSystemID)))

(event Custom|OpenGalaxyMap
  (bind _asplayership (CallFunction|GetPlayerShip))
  (Viewport|RemoveAllWidgets)
  (Utilities|ActivateLoadingScreen)
  (Utilities|IsValid _asplayership
    (:Is%20Valid
      (Class|PartGridComponent|SaveShip (Variables|/Script/Voidsinger.BaseShip|GetPartGrid _asplayership) (Variables|/Script/Voidsinger.PlayerShip|GetCurrentShipSaveSlotName _asplayership)))
    (:Is%20Not%20Valid
      _))
  (Game|OpenLevel(byObjectReference) "/Game/WorldGeneration/GalaxyMap/LVL_GalaxyMap.LVL_GalaxyMap"))

(event Custom|GenerateGalaxy
  (params (GalaxyName :type String))
  (Variables|Default|SetGalaxyName GalaxyName)
  (bind _returnvalue (SaveGame|LoadGamefromSlot GalaxyName))
  (Utilities|IsValid _returnvalue
    (:Is%20Valid
      (Variables|Default|SetGalaxySaveState (.AsBP%20Galaxy%20Map%20Save%20Data (Utilities|Casting|CastToBP_GalaxyMap_SaveData _returnvalue))))
    (:Is%20Not%20Valid
      (Variables|Default|SetGalaxySaveState 0)))
  (Class|VoidsingerGameInstance|SetPixels)
  (CallFunction|OpenGalaxyMap))

(event EventInit
  (Utilities|ActivateLoadingScreen)
  (Class|ChildClassesFinder|GenerateChildClassesMap (Variables|Default|GetChildClassFinder))
  (bind _returnvalue (UserInterface|CreateWidget "/Game/UI/UMG_Loading.UMG_Loading_C"))
  (Variables|Default|SetLoadingWidgetRef _returnvalue)
  (bind _returnvalue_2 (UserInterface|CreateWidget "/Game/UI/WorldGeneration/GalaxyMap/HUD/UMG_GalaxyMap_HUD.UMG_GalaxyMap_HUD_C"))
  (Variables|Default|SetGalaxyMap_HUD _returnvalue_2)
  (bind _returnvalue_3 (UserInterface|CreateWidget "/Game/UI/WorldGeneration/GalaxyMap/UMG_GalaxyMap_TravelArrowManager.UMG_GalaxyMap_TravelArrowManager_C"))
  (Variables|Default|SetGalaxyMap_TravelArrowManager _returnvalue_3)
  (bind _returnvalue_4 (UserInterface|CreateWidget "/Game/UI/WorldGeneration/StarSystem/HUD/UMG_StarSystem_HUD.UMG_StarSystem_HUD_C"))
  (Variables|Default|SetStarSystem_HUD _returnvalue_4)
  (bind _returnvalue_5 (UserInterface|CreateWidget "/Game/UI/BuildUI/UMG_BuildUI.UMG_BuildUI_C" (Game|GetPlayerController 0)))
  (Variables|Default|SetStarSystem_BuildUI _returnvalue_5)
  (Class|VoidsingerGameInstance|SetPixels (.Pixels (CallFunction|LoadGalaxyData)))
  (CallFunction|OpenGalaxyMap))