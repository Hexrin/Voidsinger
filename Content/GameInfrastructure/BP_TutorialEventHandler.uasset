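; Tutorial event handler, owned by the Voidsinger game instance, that shows each tutorial widget once per saved galaxy.
; Initialize loads the TutorialProgress bitmask from the galaxy save state.
; Named events for galaxy map, moving, exiting star system, voidsongs, repairing and heat application each pass a widget class and flag bit to CreateTutorialWidget.
; It skips flags already set; otherwise it adds the widget to the viewport, sets the bit and saves galaxy data.
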(event Custom|GalaxyMap
  ;[1 1 1] Galaxy Map tutorial
  (WidgetCreation|CreateTutorialWidget "/Game/UI/Tutorial/WBP_GalaxyMapTutorial.WBP_GalaxyMapTutorial_C" (|BitmaskLiteral 1)))

(event Custom|Moving
  ;[1 1 1] Moving tutorial
  (WidgetCreation|CreateTutorialWidget "/Game/UI/Tutorial/WBP_MovingTutorial.WBP_MovingTutorial_C" (|BitmaskLiteral 2)))

(event Custom|ExitingStarSystem
  ;[1 1 1] Purple Zones Tutorial
  (WidgetCreation|CreateTutorialWidget "/Game/UI/Tutorial/WBP_ExitingStarSystemTutorial.WBP_ExitingStarSystemTutorial_C" (|BitmaskLiteral 4)))

(event Custom|Voidsongs
  ;[1 1 1] Voidsongs tutorial
  (WidgetCreation|CreateTutorialWidget "/Game/UI/Tutorial/WBP_VoidsongsTutorial.WBP_VoidsongsTutorial_C" (|BitmaskLiteral 8)))

(event Custom|Reparing
  ;[1 1 1] Repairing tutorial
  (WidgetCreation|CreateTutorialWidget "/Game/UI/Tutorial/WBP_RepairingTutorial.WBP_RepairingTutorial_C" (|BitmaskLiteral 16)))

(event Custom|HeatApplication
  ;[1 1 1] Heat application tutorial
  (WidgetCreation|CreateTutorialWidget "/Game/UI/Tutorial/WBP_HeatApplicationTutorial.WBP_HeatApplicationTutorial_C" (|BitmaskLiteral 32)))

(event Custom|Initialize
  ;[1 1 1] Load tutorial progress from save state
  (Variables|Default|SetTutorialProgress (Variables|/Game/WorldGeneration/GalaxyMap/BP_GalaxyMap_SaveData.BP_GalaxyMap_SaveData_C|GetTutorialProgress (Variables|/Game/GameInfrastructure/BP_Voidsinger_GameInstance.BP_Voidsinger_GameInstance_C|GetGalaxySaveState (.AsBP%20Voidsinger%20Game%20Instance (Utilities|Casting|CastToBP_Voidsinger_GameInstance (Utilities|GetOuterObject self)))))))

(fn CreateTutorialWidget
  (params (WidgetClass :type User%20Widget%20Class%20Reference) (BitmaskFlag :type Integer))
  (bind _self self)
  (bind _returnvalue (Utilities|GetOuterObject _self))
  (bind _asbp_voidsinger_game_instance (Utilities|Casting|CastToBP_Voidsinger_GameInstance _returnvalue))
  (bind _galaxysavestate (Variables|/Game/GameInfrastructure/BP_Voidsinger_GameInstance.BP_Voidsinger_GameInstance_C|GetGalaxySaveState _asbp_voidsinger_game_instance))
  (Development|PrintString (Utilities|GetClassDisplayName WidgetClass))
  ;[1 1 1] Check if this flag has already been set, if it is, don't continue
  (if (not (Math|Conversions|ToBoolean(Integer) (Class|KismetMathLibrary|AndIntInt BitmaskFlag (Variables|Default|GetTutorialProgress))))
    ;[1 1 1] Create the widget class given
    (bind _returnvalue_2 (UserInterface|CreateWidget WidgetClass))
    (UserInterface|Viewport|AddtoViewport _returnvalue_2 0)
    ;[1 1 1] Set the tutorial progress flag
    (Variables|Default|SetTutorialProgress (Class|KismetMathLibrary|OrIntInt (Variables|Default|GetTutorialProgress) BitmaskFlag))
    ;[1 1 1] Save tutorial progress
    (CallFunction|SaveGalaxyData (Variables|/Game/WorldGeneration/GalaxyMap/BP_GalaxyMap_SaveData.BP_GalaxyMap_SaveData_C|GetStarSystemData _galaxysavestate) (Variables|/Game/WorldGeneration/GalaxyMap/BP_GalaxyMap_SaveData.BP_GalaxyMap_SaveData_C|GetCurrentStarSystemID _galaxysavestate) (Variables|/Game/WorldGeneration/GalaxyMap/BP_GalaxyMap_SaveData.BP_GalaxyMap_SaveData_C|GetGalaxyTime _galaxysavestate) (Variables|Default|GetTutorialProgress))
    (else
      (Development|PrintString "has already been set"))))