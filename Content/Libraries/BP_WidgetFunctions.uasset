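; Blueprint library of UMG widget helpers for button styling, input labels and hierarchy lookup.
; Two setters apply a texture or material to all four button brush states.
; A lookup returns the first bound key's display name for an indexed Voidsong action.
; The interface search climbs parents from the widget itself, hops through outer-of-outer to cross widget-tree boundaries, and prints an error naming I_WidgetWindowInteraction on failure.
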(fn SetButtonTexture
  (params (Target :type Button%20Object%20Reference) (Image :type Texture%202D%20Object%20Reference))
  (bind _widgetstyle (Variables|/Script/UMG.Button|GetWidgetStyle Target))
  (Utilities|Struct|SetmembersinSlateBrush (.normal _widgetstyle) Image "Image")
  (Utilities|Struct|SetmembersinSlateBrush (.hovered _widgetstyle) Image "Image")
  (Utilities|Struct|SetmembersinSlateBrush (.pressed _widgetstyle) Image "Image")
  (Utilities|Struct|SetmembersinSlateBrush (.disabled _widgetstyle) Image "Image"))

(fn SetButtonMatierial
  (params (Target :type Button%20Object%20Reference) (Image :type Material%20Interface%20Object%20Reference))
  (bind _widgetstyle (Variables|/Script/UMG.Button|GetWidgetStyle Target))
  (Utilities|Struct|SetmembersinSlateBrush (.normal _widgetstyle) Image "Image")
  (Utilities|Struct|SetmembersinSlateBrush (.hovered _widgetstyle) Image "Image")
  (Utilities|Struct|SetmembersinSlateBrush (.pressed _widgetstyle) Image "Image")
  (Utilities|Struct|SetmembersinSlateBrush (.disabled _widgetstyle) Image "Image"))

(fn GetVoidsoingInputKeyDisplayName
  (params (VoidsongInputIndex :type Integer))
  (return (Class|KismetInputLibrary|KeyGetDisplayName (.key (Utilities|Array|Get(acopy) (Class|InputSettings|GetActionMappingbyName (Class|InputSettings|GetInputSettings) (Utilities|String|StringToName (Utilities|String|Append "Voidsong" (Utilities|String|ToString(Integer) VoidsongInputIndex)))))))))

(fn GetWidgetParentImplementingInterface
  (params (Widget :type Widget%20Object%20Reference) (Interface :type Interface%20Class%20Reference))
  (bind _output_get (LocalVariables|SetWidgetToCheck Widget))
  (while (not (Utilities|DoesObjectImplementInterface _output_get Interface))
    (Utilities|IsValid (Widget|GetParent (LocalVariables|GetWidgetToCheck))
      (:Is%20Valid
        (LocalVariables|SetWidgetToCheck (Widget|GetParent (LocalVariables|GetWidgetToCheck))))
      (:Is%20Not%20Valid
        (Utilities|IsValid (.AsWidget (Utilities|Casting|CastToWidget (Utilities|GetOuterObject (Utilities|GetOuterObject (LocalVariables|GetWidgetToCheck)))))
          (:Is%20Valid
            (LocalVariables|SetWidgetToCheck (.AsWidget (Utilities|Casting|CastToWidget (Utilities|GetOuterObject (Utilities|GetOuterObject (LocalVariables|GetWidgetToCheck)))))))
          (:Is%20Not%20Valid
            (Development|PrintString 0 (Utilities|String|Append "Error: None of the parents of " (Utilities|GetDisplayName Widget) "implement I_WidgetWindowInteraction") true true "(R=1.000000,G=0.000000,B=0.000000,A=1.000000)" 6e+01)
            (return 0))))))
  (return (LocalVariables|GetWidgetToCheck)))