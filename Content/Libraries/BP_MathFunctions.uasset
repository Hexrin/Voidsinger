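; Blueprint math function library for picking uniformly distributed random points inside a circle of a given radius, centered on the origin.
; Scales the radius by the square root of a random value so points do not cluster at the center, then converts a random angle to X and Y offsets.
; Offers a global-random version and a seeded Random Stream version for repeatable results.
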(fn GetRandomPointinCircle
  (params (Radius :type Float%20%28single-precision%29))
  (LocalVariables|SetRandRadius (* Radius (Math|Float|Sqrt (Math|Random|RandomFloat))))
  (bind _output_get (LocalVariables|SetAngle (Math|Random|RandomFloatinRange 0.0 (Math|Float|MultiplybyPi 2.0))))
  (return (Math|Vector2D|MakeVector2D (* (Math|Trig|Cos(Radians) _output_get) (LocalVariables|GetRandRadius)) (* (Math|Trig|Sin(Radians) _output_get) (LocalVariables|GetRandRadius)))))

(fn GetRandomPointinCirclefromStream
  (params (Radius :type Float%20%28single-precision%29) (Stream :type Random%20Stream%20Structure%20%28by%20ref%29))
  (LocalVariables|SetRandRadius (* Radius (Math|Float|Sqrt (Math|Random|RandomFloatfromStream Stream))))
  (bind _output_get (LocalVariables|SetAngle (Math|Random|RandomFloatinRangefromStream 0.0 (Math|Float|MultiplybyPi 2.0) Stream)))
  (return (Math|Vector2D|MakeVector2D (* (Math|Trig|Cos(Radians) _output_get) (LocalVariables|GetRandRadius)) (* (Math|Trig|Sin(Radians) _output_get) (LocalVariables|GetRandRadius)))))