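; BP_GeneralFunctions is a library of shared helper functions for Voidsinger's star system and galaxy map gameplay.
; Getters return cast references to the player ship, ship player state, both game modes and the game instance.
; OpenStarSystem opens the single star system level, passing the system ID as a level option.
; GetStarSystemData looks up the game instance's current system ID in the loaded galaxy map.
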(fn GetPlayerShip
  (return (.AsBP%20Player%20Ship (Utilities|Casting|CastToBP_PlayerShip (Game|Player|GetPlayerPawn (LocalVariables|Get__WorldContext))))))

(fn GetStarSystemGameMode
  (return (.AsBP%20Star%20System%20Game%20Mode (Utilities|Casting|CastToBP_StarSystem_GameMode (Game|GetGameMode)))))

(fn GetStarSystemPlayerState
  (return (.AsShip%20Player%20State (Utilities|Casting|CastToShipPlayerState (Variables|/Script/Engine.Pawn|GetPlayerState (Game|Player|GetPlayerPawn 0))))))

(fn GetVoidsingerGameInstance
  (return (.AsBP%20Voidsinger%20Game%20Instance (Utilities|Casting|CastToBP_Voidsinger_GameInstance (Game|GetGameInstance)))))

(fn GetGalaxyMapGameMode
  (return (.AsBP%20Galaxy%20Map%20Game%20Mode (Utilities|Casting|CastToBP_GalaxyMap_GameMode (Game|GetGameMode)))))

(fn OpenStarSystem
  (params (SystemID :type String))
  (Game|OpenLevel(byObjectReference) 0 "/Game/WorldGeneration/StarSystem/LVL_StarSystem.LVL_StarSystem" true (Utilities|String|Append "?SystemID=" SystemID)))

(fn GetStarSystemData
  (return (.Value (Utilities|Map|Find (.StarSystemData (CallFunction|LoadGalaxyMap)) (Variables|/Game/GameInfrastructure/BP_Voidsinger_GameInstance.BP_Voidsinger_GameInstance_C|GetCurrentStarSystemID (CallFunction|GetVoidsingerGameInstance))))))