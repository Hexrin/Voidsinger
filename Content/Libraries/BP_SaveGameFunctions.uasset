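; Function library that saves, loads and clears persistent galaxy map and star system data through SaveGame slots.
; Each star system stores its actor data in a slot keyed by system ID, while the galaxy map stores system data and time in a slot keyed by galaxy name.
; The galaxy save is cached on the Voidsinger game instance.
; Clearing a galaxy uses its map to delete every system slot, then its own slot and cache.
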(fn SaveStarSystem
  (params (SystemID :type String) (ActorData :type Array%20of%20S%20Star%20System%20Actor%20Data%20Structures))
  (if (!= (Utilities|String|Len SystemID) 0)
    (bind _returnvalue (SaveGame|CreateSaveGameObject "/Game/WorldGeneration/StarSystem/BP_StarSystem_SaveData.BP_StarSystem_SaveData_C"))
    (Variables|/Game/WorldGeneration/StarSystem/BP_StarSystem_SaveData.BP_StarSystem_SaveData_C|SetActorData _returnvalue ActorData)
    (SaveGame|SaveGametoSlot _returnvalue (StarSystem|StarSystemSlotName SystemID))))

(fn LoadStarSystem
  (params (SystemID :type String))
  (bind _returnvalue (SaveGame|LoadGamefromSlot (StarSystem|StarSystemSlotName SystemID)))
  (Utilities|IsValid _returnvalue
    (:Is%20Valid
      (return true (Variables|/Game/WorldGeneration/StarSystem/BP_StarSystem_SaveData.BP_StarSystem_SaveData_C|GetActorData (.AsBP%20Star%20System%20Save%20Data (Utilities|Casting|CastToBP_StarSystem_SaveData _returnvalue)))))
    (:Is%20Not%20Valid
      (return false 0))))

(fn StarSystemSlotName
  (params (SystemID :type String))
  (return (Utilities|String|Append "StarSystem_" SystemID)))

(fn SaveGalaxyMap
  (params (StarSystemData :type Map%20of%20Strings%20to%20Structs) (GalaxyTime :type Float%20%28single-precision%29))
  (bind _asvoidsingergameinstance (CallFunction|GetVoidsingerGameInstance))
  (if (!= (Utilities|String|Len (Variables|/Game/GameInfrastructure/BP_Voidsinger_GameInstance.BP_Voidsinger_GameInstance_C|GetGalaxyName (CallFunction|GetVoidsingerGameInstance))) 0)
    (Utilities|IsValid (Variables|/Game/GameInfrastructure/BP_Voidsinger_GameInstance.BP_Voidsinger_GameInstance_C|GetGalaxySaveState (CallFunction|GetVoidsingerGameInstance))
      (:Is%20Valid
        _)
      (:Is%20Not%20Valid
        (bind _returnvalue (SaveGame|CreateSaveGameObject "/Game/WorldGeneration/GalaxyMap/BP_GalaxyMap_SaveData.BP_GalaxyMap_SaveData_C"))
        (Variables|/Game/GameInfrastructure/BP_Voidsinger_GameInstance.BP_Voidsinger_GameInstance_C|SetGalaxySaveState _asvoidsingergameinstance _returnvalue)))
    (Variables|/Game/WorldGeneration/GalaxyMap/BP_GalaxyMap_SaveData.BP_GalaxyMap_SaveData_C|SetGalaxyTime (Variables|/Game/GameInfrastructure/BP_Voidsinger_GameInstance.BP_Voidsinger_GameInstance_C|GetGalaxySaveState _asvoidsingergameinstance) GalaxyTime)
    (Variables|/Game/WorldGeneration/GalaxyMap/BP_GalaxyMap_SaveData.BP_GalaxyMap_SaveData_C|SetStarSystemData (Variables|/Game/GameInfrastructure/BP_Voidsinger_GameInstance.BP_Voidsinger_GameInstance_C|GetGalaxySaveState _asvoidsingergameinstance) StarSystemData)
    (SaveGame|SaveGametoSlot (Variables|/Game/GameInfrastructure/BP_Voidsinger_GameInstance.BP_Voidsinger_GameInstance_C|GetGalaxySaveState _asvoidsingergameinstance) (GalaxyMap|GalaxyMapSlotName))))

(fn LoadGalaxyMap
  (bind _asvoidsingergameinstance (CallFunction|GetVoidsingerGameInstance))
  (Utilities|IsValid (Variables|/Game/GameInfrastructure/BP_Voidsinger_GameInstance.BP_Voidsinger_GameInstance_C|GetGalaxySaveState _asvoidsingergameinstance)
    (:Is%20Valid
      (return true (Variables|/Game/WorldGeneration/GalaxyMap/BP_GalaxyMap_SaveData.BP_GalaxyMap_SaveData_C|GetStarSystemData (Variables|/Game/GameInfrastructure/BP_Voidsinger_GameInstance.BP_Voidsinger_GameInstance_C|GetGalaxySaveState _asvoidsingergameinstance)) (Variables|/Game/WorldGeneration/GalaxyMap/BP_GalaxyMap_SaveData.BP_GalaxyMap_SaveData_C|GetGalaxyTime (Variables|/Game/GameInfrastructure/BP_Voidsinger_GameInstance.BP_Voidsinger_GameInstance_C|GetGalaxySaveState _asvoidsingergameinstance))))
    (:Is%20Not%20Valid
      (bind _returnvalue (SaveGame|LoadGamefromSlot (GalaxyMap|GalaxyMapSlotName)))
      (Utilities|IsValid _returnvalue
        (:Is%20Valid
          (Variables|/Game/GameInfrastructure/BP_Voidsinger_GameInstance.BP_Voidsinger_GameInstance_C|SetGalaxySaveState _asvoidsingergameinstance (.AsBP%20Galaxy%20Map%20Save%20Data (Utilities|Casting|CastToBP_GalaxyMap_SaveData _returnvalue)))
          (return true (Variables|/Game/WorldGeneration/GalaxyMap/BP_GalaxyMap_SaveData.BP_GalaxyMap_SaveData_C|GetStarSystemData (.AsBP%20Galaxy%20Map%20Save%20Data (Utilities|Casting|CastToBP_GalaxyMap_SaveData _returnvalue))) (Variables|/Game/WorldGeneration/GalaxyMap/BP_GalaxyMap_SaveData.BP_GalaxyMap_SaveData_C|GetGalaxyTime (.AsBP%20Galaxy%20Map%20Save%20Data (Utilities|Casting|CastToBP_GalaxyMap_SaveData _returnvalue)))))
        (:Is%20Not%20Valid
          (return false 0 0.0))))))

(fn GalaxyMapSlotName
  (return (Utilities|String|Append "GalaxyMap_" (Variables|/Game/GameInfrastructure/BP_Voidsinger_GameInstance.BP_Voidsinger_GameInstance_C|GetGalaxyName (CallFunction|GetVoidsingerGameInstance)))))

(fn ClearAllStarSystemData
  (bind (_galaxyfound _starsystemdata) (GalaxyMap|LoadGalaxyMap))
  (if _galaxyfound
    (bind _values (Utilities|Map|Values _starsystemdata))
    (for _array_element _values
      (SaveGame|DeleteGameinSlot (StarSystem|StarSystemSlotName (.systemid _array_element))))))

(fn ClearGalaxyData
  (StarSystem|ClearAllStarSystemData)
  (SaveGame|DeleteGameinSlot (GalaxyMap|GalaxyMapSlotName))
  (Variables|/Game/GameInfrastructure/BP_Voidsinger_GameInstance.BP_Voidsinger_GameInstance_C|SetGalaxySaveState (CallFunction|GetVoidsingerGameInstance) 0))