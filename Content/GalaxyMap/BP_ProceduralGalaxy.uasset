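; Galaxy map actor that procedurally scatters stars along a spline on BeginPlay.
; It steps along the spline by StarSpawnDistance, sampling a vector curve by normalized distance: Z sets star probability, X and Y bound the random right and left offset.
; PercentofStarsVisitable decides whether each star becomes a spawned BP_VisitableStar actor, raised slightly in Z, or a static mesh component added to this actor.
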(event EventBeginPlay
  (bind _spline (Variables|Default|GetSpline))
  (bind _starspawndistance (Variables|Default|GetStarSpawnDistance))
  (bind _returnvalue (Spline|GetSplineLength _spline))
  (for _index (range 0 (Math|Float|Truncate (/ _returnvalue _starspawndistance)))
    (if (Math|Random|RandomBoolwithWeight (.z (Math|Curves|GetVectorValue (Variables|Default|GetCurve) (/ (* _index _starspawndistance) _returnvalue))))
      (if (Math|Random|RandomBoolwithWeight (Variables|Default|GetPercentofStarsVisitable))
        (Game|SpawnActorfromClass "/Game/GalaxyMap/BP_VisitableStar.BP_VisitableStar_C" (Math|Transform|MakeTransform (+ (Transformation|GetActorLocation) (+ (Spline|GetLocationatDistanceAlongSpline _spline (* _index _starspawndistance) "Local") (* (Math|Random|RandomFloatinRange (* (.y (Math|Curves|GetVectorValue (Variables|Default|GetCurve) (/ (* _index _starspawndistance) _returnvalue))) -1.0) (.x (Math|Curves|GetVectorValue (Variables|Default|GetCurve) (/ (* _index _starspawndistance) _returnvalue)))) (Class|SplineComponent|GetRightVectoratDistanceAlongSpline _spline (* _index _starspawndistance) "Local"))) "0.000000,0.000000,1.000000") "0, 0, 0" "1,1,1") "Undefined" 0 0)
        (else
          (AddComponent|AddStaticMeshComponent false (Math|Transform|MakeTransform (+ (Spline|GetLocationatDistanceAlongSpline _spline (* _index _starspawndistance) "Local") (* (Math|Random|RandomFloatinRange (* (.y (Math|Curves|GetVectorValue (Variables|Default|GetCurve) (/ (* _index _starspawndistance) _returnvalue))) -1.0) (.x (Math|Curves|GetVectorValue (Variables|Default|GetCurve) (/ (* _index _starspawndistance) _returnvalue)))) (Class|SplineComponent|GetRightVectoratDistanceAlongSpline _spline (* _index _starspawndistance) "Local"))) "0, 0, 0" "1,1,1")))))))

(fn ConstructionScript)