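; Player ship Blueprint with keyboard controls for editing its part grid and pushing it, and a galaxy map widget shown on BeginPlay.
; Arrow keys step a shared Location coordinate, and each step moves the SelectionIndicator to that spot.
; T adds an unrotated Hull part to PartGrid at Location, while G applies a fixed X-axis force through MovementComponent at the same point.
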(event EventTick
  (params (DeltaSeconds :type Float%20%28single-precision%29)))

(event EventBeginPlay
  (bind _returnvalue (UserInterface|CreateWidget "/Game/GalaxyMap/GalaxyMap.GalaxyMap_C"))
  (UserInterface|Viewport|AddtoViewport _returnvalue 0))

(event Input|KeyboardEvents|T
  (params (Key :type Key%20Structure :default "None"))
  (:Pressed
    (Class|PartGridComponent|AddPart (Variables|Default|GetPartGrid) "/Game/Parts/Hull.Hull_C" (Variables|Default|GetLocation) "Degrees0" false)))

(event Input|KeyboardEvents|Left
  (params (Key :type Key%20Structure :default "None"))
  (:Pressed
    (Math|Integer|DecrementInt (.x (Variables|Default|GetLocation))
      (:%20%20
        (Transformation|SetRelativeLocation (Variables|Default|GetSelectionIndicator) (Math|Conversions|ToVector(Vector2D) (Math|Conversions|ToVector2D(IntPoint) (Variables|Default|GetLocation))) false false)))))

(event Input|KeyboardEvents|Right
  (params (Key :type Key%20Structure :default "None"))
  (:Pressed
    (Math|Integer|IncrementInt (.x (Variables|Default|GetLocation))
      (:%20%20
        (Transformation|SetRelativeLocation (Variables|Default|GetSelectionIndicator) (Math|Conversions|ToVector(Vector2D) (Math|Conversions|ToVector2D(IntPoint) (Variables|Default|GetLocation))) false false)))))

(event Input|KeyboardEvents|Up
  (params (Key :type Key%20Structure :default "None"))
  (:Pressed
    (Math|Integer|IncrementInt (.y (Variables|Default|GetLocation))
      (:%20%20
        (Transformation|SetRelativeLocation (Variables|Default|GetSelectionIndicator) (Math|Conversions|ToVector(Vector2D) (Math|Conversions|ToVector2D(IntPoint) (Variables|Default|GetLocation))) false false)))))

(event Input|KeyboardEvents|Down
  (params (Key :type Key%20Structure :default "None"))
  (:Pressed
    (Math|Integer|DecrementInt (.y (Variables|Default|GetLocation))
      (:%20%20
        (Transformation|SetRelativeLocation (Variables|Default|GetSelectionIndicator) (Math|Conversions|ToVector(Vector2D) (Math|Conversions|ToVector2D(IntPoint) (Variables|Default|GetLocation))) false false)))))

(event Input|KeyboardEvents|G
  (params (Key :type Key%20Structure :default "None"))
  (:Pressed
    (Class|ShipMovementComponent|AddForce (Variables|Default|GetMovementComponent) (Math|Conversions|ToVector2D(IntPoint) (Variables|Default|GetLocation)) "(X=10.000000,Y=0.000000)")))

(fn ConstructionScript)