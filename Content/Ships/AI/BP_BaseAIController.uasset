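; Base AI controller for BaseShip pawns that runs a behavior tree and exposes move direction, deceleration and look direction events.
; MoveToPoint opens a Tick gate that turns the ship toward the target and drives it forward.
; It brakes when a velocity-based fudge estimate nears or exceeds remaining distance, nudges forward if stopped short, and closes the gate once stopped within tolerance.
; The sight perception handler is empty.
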(event OnPerceptionUpdated(Sight)
  (params (UpdatedActors :type Array%20of%20Actor%20Object%20References))
  ;[1 0 0 0.277 117] Needs Comments - Liam Suggestion
  ;;[1 0 0] Delete Unused Code - Liam Suggestion
)

(event Custom|SetMoveDirection
  (params (MoveDirection :type Vector%202D%20Structure) (ControlledPawn :type Pawn%20Object%20Reference))
  ;[1 0 0 0.277 117] Needs Comments - Liam Suggestion
  ;;[1 0 0] Why does both this and the task that does the same thing exist?
  ;;  - Liam Suggestion
  (Class|BaseShip|SetTargetMoveDirection (.AsBase%20Ship (Utilities|Casting|CastToBaseShip ControlledPawn)) MoveDirection))

(event Custom|SetDecelerating
  (params (Decelerating :type Boolean) (ControlledPawn :type Pawn%20Object%20Reference))
  ;[1 0 0 0.277 117] Needs Comments - Liam Suggestion
  ;;[1 0 0] Why does both this and the task that does the same thing exist?
  ;;  - Liam Suggestion
  (Class|BaseShip|SetTargetMoveSpeed (.AsBase%20Ship (Utilities|Casting|CastToBaseShip ControlledPawn)) (select Decelerating 0.0 (Variables|Default|GetMaxTargetSpeed))))

(event Custom|SetLookDirection
  (params (LookDirection :type Vector) (ControlledPawn :type Pawn%20Object%20Reference))
  ;[1 0 0 0.277 117] Needs Comments - Liam Suggestion
  ;;[1 0 0] Why does both this and the task that does the same thing exist?
  ;;  - Liam Suggestion
  (Class|BaseShip|SetTargetLookDirection (.AsBase%20Ship (Utilities|Casting|CastToBaseShip ControlledPawn)) LookDirection))

(event Custom|MoveToPoint
  (params (Location :type Vector%202D%20Structure) (ControlledPawn :type Pawn%20Object%20Reference))
  (bind _returnvalue (Transformation|GetActorLocation ControlledPawn))
  (bind _asbase_ship (Utilities|Casting|CastToBaseShip ControlledPawn))
  (bind _asbase_ship_2 (Utilities|Casting|CastToBaseShip ControlledPawn))
  (bind _decelerationfudgetolerancemultiplier (Variables|Default|GetDecelerationFudgeToleranceMultiplier))
  (bind _returnvalue_2 (- Location _returnvalue))
  (bind _physicscomponent (Variables|/Script/Voidsinger.BaseShip|GetPhysicsComponent _asbase_ship_2))
  (bind _physicscomponent_2 (Variables|/Script/Voidsinger.BaseShip|GetPhysicsComponent _asbase_ship))
  (bind _returnvalue_3 (Class|ShipPhysicsComponent|GetVelocity _physicscomponent))
  (bind _returnvalue_4 (Math|Vector|VectorLength _returnvalue_2))
  (bind _returnvalue_5 (Class|ShipPhysicsComponent|GetVelocity _physicscomponent_2))
  (bind _returnvalue_6 (Class|KismetMathLibrary|GetAbs2D _returnvalue_3))
  (bind _returnvalue_7 (Utilities|Operators|EqualEqual _returnvalue_5 "(X=0.000000,Y=0.000000)" 1.0))
  (bind _returnvalue_8 (* (.x _returnvalue_6) (.y _returnvalue_6) _decelerationfudgetolerancemultiplier))
  ;[1 0 0 0.277 117] Needs Comments - Liam Suggestion
  ;;[1 0 0 1 15] Overcomplcated.
  ;; Logic should be as follows:
  ;; //On Tick:
  ;; TargetMoveDirection = [Direction from pawn to Location]
  ;; if ([Pawn Location] (Not aproximatly equal) TargetPoint])
  ;; {
  ;;      if ([time to point] > [time to 0 velocity])
  ;;      {
  ;;           TargetMoveSpeed = 0
  ;;      } else {
  ;;           TargetMoveSpeed = MoveSpeed
  ;;      }
  ;; }
  ;;
  ;;
  ;; This should be in the MoveToPoint Task.
  ;;  - Liam Suggestion
  (if (.AIDebug (Utilities|GetClassDefaults "/Game/DebugSettings.DebugSettings_C"))
    (Rendering|Debug|DrawDebugPoint (Math|Conversions|ToVector(Vector2D) Location) 5.0 "(R=1.000000,G=0.159665,B=0.000000,A=1.000000)" 1234.0))
  (CallFunction|SetMoveDirection "(X=1.000000,Y=0.000000)" ControlledPawn)
  (CallFunction|SetDecelerating false ControlledPawn)
  (Variables|Default|SetUseStoppingFudge false)
  (Utilities|FlowControl|Gate true) ; enters at Open
)

(event EventBeginPlay
  ;[1 0 0 0.277 117] Needs Comments - Liam Suggestion
  (AI|RunBehaviorTree (Variables|Default|GetBTAsset)))

(event EventTick
  (params (DeltaSeconds :type Float%20%28single-precision%29))
  ;[1 0 0 0.277 117] Needs Comments - Liam Suggestion
  ;;[1 0 0 1 15] Overcomplcated.
  ;; Logic should be as follows:
  ;; //On Tick:
  ;; TargetMoveDirection = [Direction from pawn to Location]
  ;; if ([Pawn Location] (Not aproximatly equal) TargetPoint])
  ;; {
  ;;      if ([time to point] > [time to 0 velocity])
  ;;      {
  ;;           TargetMoveSpeed = 0
  ;;      } else {
  ;;           TargetMoveSpeed = MoveSpeed
  ;;      }
  ;; }
  ;;
  ;;
  ;; This should be in the MoveToPoint Task.
  ;;  - Liam Suggestion
  (Utilities|FlowControl|Gate true :!label _label
    (:Exit
      (CallFunction|SetLookDirection (- (stale Custom|MoveToPoint Location) (Transformation|GetActorLocation (stale Custom|MoveToPoint ControlledPawn))) (stale Custom|MoveToPoint ControlledPawn))
      (if (or (Math|Float|NearlyEqual(Float) (Math|Vector|VectorLength (- (stale Custom|MoveToPoint Location) (Transformation|GetActorLocation (stale Custom|MoveToPoint ControlledPawn)))) (* (.x (Class|KismetMathLibrary|GetAbs2D (Class|ShipPhysicsComponent|GetVelocity (Variables|/Script/Voidsinger.BaseShip|GetPhysicsComponent (.AsBase%20Ship (Utilities|Casting|CastToBaseShip (stale Custom|MoveToPoint ControlledPawn))))))) (.y (Class|KismetMathLibrary|GetAbs2D (Class|ShipPhysicsComponent|GetVelocity (Variables|/Script/Voidsinger.BaseShip|GetPhysicsComponent (.AsBase%20Ship (Utilities|Casting|CastToBaseShip (stale Custom|MoveToPoint ControlledPawn))))))) (Variables|Default|GetDecelerationFudgeToleranceMultiplier)) (Math|Float|SelectFloat (Variables|Default|GetStoppingFudgeTolerance) (+ (Variables|Default|GetStartDeceleratingDistance) (Variables|Default|GetDecelerationFudgeTolerance)) (Variables|Default|GetUseStoppingFudge))) (> (* (.x (Class|KismetMathLibrary|GetAbs2D (Class|ShipPhysicsComponent|GetVelocity (Variables|/Script/Voidsinger.BaseShip|GetPhysicsComponent (.AsBase%20Ship (Utilities|Casting|CastToBaseShip (stale Custom|MoveToPoint ControlledPawn))))))) (.y (Class|KismetMathLibrary|GetAbs2D (Class|ShipPhysicsComponent|GetVelocity (Variables|/Script/Voidsinger.BaseShip|GetPhysicsComponent (.AsBase%20Ship (Utilities|Casting|CastToBaseShip (stale Custom|MoveToPoint ControlledPawn))))))) (Variables|Default|GetDecelerationFudgeToleranceMultiplier)) (Math|Vector|VectorLength (- (stale Custom|MoveToPoint Location) (Transformation|GetActorLocation (stale Custom|MoveToPoint ControlledPawn))))))
        (CallFunction|SetDecelerating true (stale Custom|MoveToPoint ControlledPawn))
        (if (Math|Vector|VectorIsNearlyZero (- (stale Custom|MoveToPoint Location) (Transformation|GetActorLocation (stale Custom|MoveToPoint ControlledPawn))) (Variables|Default|GetStoppingFudgeTolerance))
          (if (Utilities|Operators|EqualEqual (Class|ShipPhysicsComponent|GetVelocity (Variables|/Script/Voidsinger.BaseShip|GetPhysicsComponent (.AsBase%20Ship (Utilities|Casting|CastToBaseShip (stale Custom|MoveToPoint ControlledPawn))))) "(X=0.000000,Y=0.000000)" 1.0)
            (CallFunction|SetDecelerating true (stale Custom|MoveToPoint ControlledPawn))
            (goto _label Close))
          (elif (Utilities|Operators|EqualEqual (Class|ShipPhysicsComponent|GetVelocity (Variables|/Script/Voidsinger.BaseShip|GetPhysicsComponent (.AsBase%20Ship (Utilities|Casting|CastToBaseShip (stale Custom|MoveToPoint ControlledPawn))))) "(X=0.000000,Y=0.000000)" 1.0)
            (CallFunction|SetDecelerating false (stale Custom|MoveToPoint ControlledPawn))
            (CallFunction|SetMoveDirection "(X=1.000000,Y=0.000000)" (stale Custom|MoveToPoint ControlledPawn))
            (Variables|Default|SetUseStoppingFudge true)))
        (else
          (CallFunction|SetDecelerating false (stale Custom|MoveToPoint ControlledPawn))
          (CallFunction|SetMoveDirection "(X=1.000000,Y=0.000000)" (stale Custom|MoveToPoint ControlledPawn))
          (if (Variables|Default|GetUseStoppingFudge)
            (Utilities|FlowControl|Delay (Variables|Default|GetCorrectionDuration))
            (Variables|Default|SetUseStoppingFudge false)))))))

(fn ConstructionScript)