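; Behavior tree task for AI ships that, by its name, makes a ship circle the player.
; Each AI tick writes the unit direction from the ship to the player's ship into the LookDirection blackboard key.
; It also copies MoveDirection from BP_FlyAIController into the matching key, so the movement path itself is decided outside this task.
; The task has no execute event and never calls finish.
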(event EventReceiveTickAI
  (params (OwnerController :type AI%20Controller%20Object%20Reference) (ControlledPawn :type Pawn%20Object%20Reference) (DeltaSeconds :type Float%20%28single-precision%29))
  (AI|BehaviorTree|SetBlackboardValueasVector (Variables|Default|GetLookDirection) (Math|Vector|GetUnitDirection(Vector) (Transformation|GetActorLocation ControlledPawn) (Transformation|GetActorLocation (.AsBP%20Player%20Ship (Utilities|Casting|CastToBP_PlayerShip (Pawn|GetControlledPawn (Game|GetPlayerController 0)))))))
  (AI|BehaviorTree|SetBlackboardValueasVector (Variables|Default|GetMoveDirection) (Variables|/Game/Ships/AI/FlyAI/BP_FlyAIController.BP_FlyAIController_C|GetMoveDirection (.AsBP%20Fly%20AIController (Utilities|Casting|CastToBP_FlyAIController OwnerController)))))