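; Behavior tree task for ship AI that passes a blackboard move direction to the AI controller.
; On execute it reads the MoveDirection vector, converts it to 2D and calls SetMoveDirection on BP_BaseAIController for the controlled pawn, then finishes with success immediately.
; It also draws a debug arrow of the direction rotated by the pawn's rotation and prints the vector on screen.
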(event EventReceiveExecuteAI
  (params (OwnerController :type AI%20Controller%20Object%20Reference) (ControlledPawn :type Pawn%20Object%20Reference))
  (bind _returnvalue (Transformation|GetActorLocation ControlledPawn))
  (bind _movedirection (Variables|Default|GetMoveDirection))
  (bind _returnvalue_2 (Class|BTFunctionLibrary|GetBlackboardValueasVector _movedirection))
  (Default|SetMoveDirection (.AsBP%20Base%20AIController (Utilities|Casting|CastToBP_BaseAIController OwnerController)) (Math|Conversions|ToVector2D(Vector) _returnvalue_2) ControlledPawn)
  (Rendering|Debug|DrawDebugArrow _returnvalue (+ _returnvalue (* (Math|Vector|RotateVector _returnvalue_2 (Transformation|GetActorRotation ControlledPawn)) 1e+02)) 2e+01 "(R=1.000000,G=0.982410,B=0.000000,A=1.000000)" 0.1 2.0)
  (Development|PrintString (Utilities|String|ToString(Vector) _returnvalue_2) true true "(R=1.000000,G=0.000000,B=0.000000,A=1.000000)" 0.0)
  (AI|BehaviorTree|FinishExecute true))