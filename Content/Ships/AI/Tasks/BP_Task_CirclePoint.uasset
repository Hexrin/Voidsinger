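; Behavior tree task that steers an AI ship around the player ship on a circular path.
; On tick, it advances a yaw angle at one revolution per EnemyCycle and rotates the EnemyDistance offset by it.
; It adds that offset and the player's velocity to the player's location as a lead, sends the 2D point to the AI controller's MoveToPoint, then finishes successfully.
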(event EventReceiveTickAI
  (params (OwnerController :type AI%20Controller%20Object%20Reference) (ControlledPawn :type Pawn%20Object%20Reference) (DeltaSeconds :type Float%20%28single-precision%29))
  (bind _returnvalue (Game|GetPlayerController 0))
  (bind _returnvalue_2 (Pawn|GetControlledPawn _returnvalue))
  (bind _asbp_player_ship (Utilities|Casting|CastToBP_PlayerShip _returnvalue_2))
  (Variables|Default|SetTimer (+ (Variables|Default|GetTimer) (* DeltaSeconds (/ 3.6e+02 (Variables|Default|GetEnemyCycle)))))
  (Default|MovetoPoint (.AsBP%20Base%20AIController (Utilities|Casting|CastToBP_BaseAIController OwnerController)) (Math|Conversions|ToVector2D(Vector) (+ (Transformation|GetActorLocation _asbp_player_ship) (Math|Vector|RotateVector (Variables|Default|GetEnemyDistance) (Math|Rotator|MakeRotator 0.0 0.0 (Variables|Default|GetTimer))) (Class|ShipPhysicsComponent|GetVelocity (Variables|/Script/Voidsinger.BaseShip|GetPhysicsComponent _asbp_player_ship)))) ControlledPawn)
  (AI|BehaviorTree|FinishExecute true))