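; Behavior tree task that makes an enemy ship wander by periodically picking a new random movement direction.
; On AI tick, it shifts an accumulated angle by up to 45 degrees either way and rotates the world X axis by it.
; The flat vector goes to the MoveDirection blackboard key and the ship's MoveDirection.
; A gate and Delay limit changes to about every five seconds; the task never calls Finish Execute.
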(event EventReceiveTickAI
  (params (OwnerController :type AI%20Controller%20Object%20Reference) (ControlledPawn :type Pawn%20Object%20Reference) (DeltaSeconds :type Float%20%28single-precision%29))
  (bind _returnvalue (Transformation|GetActorLocation ControlledPawn))
  (Utilities|FlowControl|Sequence
    (:then_0
      (Utilities|FlowControl|Gate false :!label _label
        (:Exit
          (bind _output_get (Variables|Default|SetCurrentAngle (+ (Variables|Default|GetCurrentAngle) (Math|Float|Lerp 45.0 -45.0 (Math|Random|RandomFloat)))))
          (AI|BehaviorTree|SetBlackboardValueasVector (Variables|Default|GetMoveDirection) (Math|Conversions|ToVector(Vector2D) (Class|KismetMathLibrary|GetRotated2D (Math|Conversions|ToVector2D(Vector) (Math|Vector|GetUnitDirection(Vector) _returnvalue (+ _returnvalue "1.000000,0,0"))) _output_get)))
          (Variables|/Game/Ships/BP_BaseEnemyShip.BP_BaseEnemyShip_C|SetMoveDirection (.AsBP%20Base%20Enemy%20Ship (Utilities|Casting|CastToBP_BaseEnemyShip ControlledPawn)) (Math|Conversions|ToVector(Vector2D) (Class|KismetMathLibrary|GetRotated2D (Math|Conversions|ToVector2D(Vector) (Math|Vector|GetUnitDirection(Vector) _returnvalue (+ _returnvalue "1.000000,0,0"))) _output_get)))
          (goto _label Close))))
    (:then_1
      (Utilities|FlowControl|Delay 5.0)
      (goto _label Open))))