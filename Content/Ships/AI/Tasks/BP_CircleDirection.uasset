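; BP_CircleDirection is a behavior tree task for flying ship AI that steers the pawn around a fixed point.
; On first tick it stores a point offset from the pawn's start, then each tick writes the look direction toward it to the blackboard.
; It also sets a constant forward-and-sideways move direction and target speed on the controller, copying the direction to the blackboard.
; The distance check has no effect, and a debug point marks the center.
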(event EventReceiveTickAI
  (params (OwnerController :type AI%20Controller%20Object%20Reference) (ControlledPawn :type Pawn%20Object%20Reference) (DeltaSeconds :type Float%20%28single-precision%29))
  (bind _returnvalue (Transformation|GetActorLocation ControlledPawn))
  (bind _asbp_fly_aicontroller (Utilities|Casting|CastToBP_FlyAIController OwnerController))
  (Utilities|FlowControl|Sequence
    (:then_0
      (Utilities|FlowControl|DoOnce false
        (:Completed
          (bind _output_get (Variables|Default|SetInitialPointLocation (- _returnvalue "0,100.000000,0"))))))
    (:then_1
      (AI|BehaviorTree|SetBlackboardValueasVector (Variables|Default|GetLookDirection) (Math|Vector|GetUnitDirection(Vector) _returnvalue (Variables|Default|GetInitialPointLocation)))
      (Rendering|Debug|DrawDebugPoint _output_get 1e+01 "(R=0.020638,G=1.000000,B=0.000000,A=1.000000)" 0.0)
      (if (> (Math|Vector|Distance2D(Vector) (Math|Conversions|ToVector2D(Vector) _returnvalue) (Math|Conversions|ToVector2D(Vector) (Variables|Default|GetInitialPointLocation))) 1e+02)
        _
        (else
          _))
      (Variables|/Game/Ships/AI/FlyAI/BP_FlyAIController.BP_FlyAIController_C|SetMoveDirection _asbp_fly_aicontroller "1.000000,0.800000, 0")
      (Variables|/Game/Ships/AI/BP_BaseAIController.BP_BaseAIController_C|SetTargetmoveSpeed (.AsBP%20Base%20AIController (Utilities|Casting|CastToBP_BaseAIController OwnerController)) 5e+01)
      (AI|BehaviorTree|SetBlackboardValueasVector (Variables|Default|GetMoveDirection) (Variables|/Game/Ships/AI/FlyAI/BP_FlyAIController.BP_FlyAIController_C|GetMoveDirection _asbp_fly_aicontroller)))))