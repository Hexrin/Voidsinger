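; Behavior tree service for AI ships that flags when the player's ship is within range.
; Each AI tick it compares the 2D distance between the controlled pawn and the player ship against PlayerRange, ignoring height.
; Inside that range it sets the MoveBack blackboard key and raises the AI controller's target move speed.
; Otherwise it clears the key and applies the lower speed.
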(event EventReceiveTickAI
  (params (OwnerController :type AI%20Controller%20Object%20Reference) (ControlledPawn :type Pawn%20Object%20Reference) (DeltaSeconds :type Float%20%28single-precision%29))
  (bind _asbp_base_aicontroller (Utilities|Casting|CastToBP_BaseAIController OwnerController))
  (bind _moveback (Variables|Default|GetMoveBack))
  (if (< (Math|Vector|Distance2D(Vector) (Math|Conversions|ToVector2D(Vector) (Transformation|GetActorLocation ControlledPawn)) (Math|Conversions|ToVector2D(Vector) (Transformation|GetActorLocation (.AsBP%20Player%20Ship (Utilities|Casting|CastToBP_PlayerShip (Pawn|GetControlledPawn (Game|GetPlayerController 0))))))) (Variables|Default|GetPlayerRange))
    (Class|BTFunctionLibrary|SetBlackboardValueasBool _moveback true)
    (Variables|/Game/Ships/AI/BP_BaseAIController.BP_BaseAIController_C|SetTargetmoveSpeed _asbp_base_aicontroller 1.5e+02)
    (else
      (Class|BTFunctionLibrary|SetBlackboardValueasBool _moveback false)
      (Variables|/Game/Ships/AI/BP_BaseAIController.BP_BaseAIController_C|SetTargetmoveSpeed _asbp_base_aicontroller 1e+02))))