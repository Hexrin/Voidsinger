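; Ship part Blueprint for electricity storage, with all of its logic in BeginPlay.
; It continues only if its part grid's owner is a BaseShip, then debug-prints the Electricity system's resource amount.
; If that amount is at or above a hardcoded threshold, it adds the negated amount, emptying the system.
; Inline review comments question the cast, threshold, drain and leftover debug print.
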(event EventBeginPlay
  (bind _returnvalue (Class|BasePart|GetSystembyType "Electricity"))
  (bind _returnvalue_2 (Class|BaseResourceSystem|GetResourceAmount _returnvalue))
  ;[0 0.3961 0.03922] Why is this here? this should always be true -Mabel
  (Utilities|Casting|CastToBaseShip (Components|GetOwner (Class|BasePart|GetPartGrid)))
  ;[0 0.3961 0.03922] Remember to remove debug stuff or put it behind a boolean when you're finished with it -Mabel
  (Development|PrintString (Utilities|String|ToString(Float) _returnvalue_2) true true "(R=0.000000,G=0.190620,B=1.000000,A=1.000000)" 0.0)
  (if (>= _returnvalue_2 3e+01)
    ;[0 0.3961 0.03922] Why does this remove all the fuel when the fuel amount is greater than 30? -Mabel
    (Class|BaseResourceSystem|AddResources _returnvalue (* _returnvalue_2 -1.0))))