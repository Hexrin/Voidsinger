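; Thruster ship part that drives an exhaust effect and heat-damages ship parts caught behind it.
; BeginPlay attaches a Niagara gas system to the ship; each tick updates its position, ship velocity and throttle, zeroed when fuel is nearly empty.
; A per-tick box trace behind the nozzle applies throttle- and time-scaled heat to hit BaseShip part grids.
; On destruction, the effect's throttle drops to zero.
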(event EventOnDestroyed
  ;[0.2448 0.2448 0.2448] This Function traces a line behind the thruster when it is fired and spawns a system, then applies heat damage to al parts in the trace.
  ;;[1 1 1] Destroys the Effect when destroyed
  (Niagara|SetNiagaraVariable(Float) (Variables|Default|GetSystemRef) "Throttle" 0.0))

(event EventBeginPlay
  ;[0.2448 0.2448 0.2448] This Function traces a line behind the thruster when it is fired and spawns a system, then applies heat damage to al parts in the trace.
  ;;[1 0.09375 0.09375] Spawns Niagra System for the Thruster Particle Effect
  (bind _returnvalue (Game|AddComponentbyClass (Class|BasePart|GetShip) "/Script/Niagara.NiagaraComponent" false (Math|Transform|MakeTransform (Math|Conversions|ToVector(Vector2D) (Class|BaseThrusterPart|GetThrustRelativeLocation)) (Math|Rotator|MakeRotator 0.0 0.0 (Class|BaseThrusterPart|GetThrustRotation)) "1,1,1")))
  (Class|NiagaraComponent|SetAsset _returnvalue "/Game/FX/NS_Thruster_Gas.NS_Thruster_Gas")
  (Variables|Default|SetSystemRef _returnvalue))

(event EventOnTick
  (params (DeltaTime :type Float%20%28single-precision%29))
  (bind _returnvalue (Class|BaseThrusterPart|GetThrottle))
  (bind _returnvalue_2 (Class|BasePart|GetSystembyType "Fuel"))
  (bind _systemref (Variables|Default|GetSystemRef))
  (bind _systemref_2 (Variables|Default|GetSystemRef))
  (bind _fuelconsumptionrate (Variables|Default|GetFuelConsumptionRate))
  (bind _returnvalue_3 (Transformation|GetWorldLocation _systemref_2))
  (bind _returnvalue_4 (Class|BaseResourceSystem|GetResourceAmount _returnvalue_2))
  (bind _returnvalue_5 (Transformation|GetWorldRotation _systemref_2))
  (bind _returnvalue_6 (Math|Conversions|ToVector2D(Vector) _returnvalue_3))
  (bind _returnvalue_7 (Math|Float|NearlyEqual(Float) _returnvalue_4 0.0 _fuelconsumptionrate))
  (bind _returnvalue_8 (Math|Conversions|ToVector(Vector2D) _returnvalue_6))
  (bind _returnvalue_9 (select _returnvalue_7 0.0 _returnvalue))
  ;[0.2448 0.2448 0.2448] This Function traces a line behind the thruster when it is fired and spawns a system, then applies heat damage to al parts in the trace.
  ;;[1 0.9412 0] Logic to set the Velocity attribute in the system
  (Transformation|SetRelativeLocation _systemref (Math|Conversions|ToVector(Vector2D) (Class|BaseThrusterPart|GetThrustRelativeLocation)) false false)
  (Niagara|SetNiagaraVariable(Vector3) _systemref "Velocity" (Math|Conversions|ToVector(Vector2D) (Class|ShipPhysicsComponent|GetVelocity (Variables|/Script/Voidsinger.BaseShip|GetPhysicsComponent (Class|BasePart|GetShip)))))
  ;;[0.05647 1 0.09381] Logic on setting the attribute inside of the niagara system
  (Niagara|SetNiagaraVariable(Float) _systemref "Throttle" _returnvalue_9)
  ;;[1 0 0.821] Trace and Applying Heat to parts in the trace
  (bind _outhits (Class|KismetSystemLibrary|BoxTraceMulti _returnvalue_8 (+ _returnvalue_8 (* (Math|Rotator|GetRotationXVector _returnvalue_5) -15.625)) (Variables|Default|GetHalf%20Size) _returnvalue_5 "TraceTypeQuery1" false 0 "None" false))
  (for _array_element _outhits
    (if (and (.bblockinghit _array_element) (.bSuccess (Utilities|Casting|CastToBaseShip (.hitactor _array_element))))
      (Class|PartGridComponent|ApplyHeatatLocation (Variables|/Script/Voidsinger.BaseShip|GetPartGrid (.AsBase%20Ship (Utilities|Casting|CastToBaseShip (.hitactor _array_element)))) (- (.impactpoint _array_element) (* (.normal _array_element) 1.0)) (* (Variables|Default|GetThrustDamage) DeltaTime _returnvalue_9)))))