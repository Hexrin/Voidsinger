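; BP_AmmoManufacturer is a part that converts electricity into ammo at a set production rate.
; A looping timer started on BeginPlay draws a per-cycle share of power from the Electricity system and, on success, adds one unit to the Ammo system, with a debug print.
; Critical damage triggers a one-time explosion at the part's location and pauses the production timer.
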(event Custom|ProduceAmmo
  (bind _returnvalue (Class|BaseResourceSystem|DrawResources (Class|BasePart|GetSystembyType "Electricity") (/ (Variables|Default|GetElectricityComsumtionRate) (Variables|Default|GetAmmoProductionRate))))
  (if _returnvalue
    (Development|PrintString "Hello")
    (Class|BaseResourceSystem|AddResources (Class|BasePart|GetSystembyType "Ammo") 1.0)))

(event EventOnCriticallyDamaged
  (Utilities|FlowControl|DoOnce false
    (:Completed
      (Class|FunctionLibrary|ExplodeatWorldLocation (Class|BasePart|GetPartWorldLocation) (Variables|Default|GetExplosion%20Radius))
      (Utilities|Time|PauseTimerbyHandle (stale EventBeginPlay _returnvalue)))))

(event EventBeginPlay
  (bind _returnvalue (Utilities|Time|SetTimerbyEvent (delegate Custom|ProduceAmmo) (/ 1.0 (Variables|Default|GetAmmoProductionRate)) true 1.0)))