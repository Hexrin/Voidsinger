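; BP_Core is the ship core part: its critical damage reports player death, or pays pixels and fuel for an enemy kill.
; Activation opens a gate that runs an overlap scan each tick until the game mode's Voidsong deactivation closes it.
; The scan sizes a sphere from the part grid bounds and steps through grid offsets on overlapped actors.
; It is unfinished: only debug draws and prints remain, with the ActivateWithEffects call disconnected.
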(event Custom|Deactivate
  (bind _returnvalue (Class|BasePart|GetPartWorldLocation))
  (bind _self self)
  (bind _returnvalue_2 (Utilities|GetOuterObject _self))
  (bind _aspart_grid_component (Utilities|Casting|CastToPartGridComponent _returnvalue_2))
  (bind _returnvalue_3 (Class|PartGridComponent|GetPartGridBounds _aspart_grid_component))
  (bind _returnvalue_4 (Math|Conversions|ToVector2D(IntPoint) (.upperbounds _returnvalue_3)))
  (bind _returnvalue_5 (Math|Conversions|ToVector2D(IntPoint) (.lowerbounds _returnvalue_3)))
  (bind _returnvalue_6 (Math|Vector2D|Vector2DLength _returnvalue_4))
  (bind _returnvalue_7 (Class|KismetMathLibrary|VSize2DSquared _returnvalue_4))
  (bind _returnvalue_8 (Class|KismetMathLibrary|VSize2DSquared _returnvalue_5))
  (bind _returnvalue_9 (Math|Vector2D|Vector2DLength _returnvalue_5))
  (bind _returnvalue_10 (> _returnvalue_8 _returnvalue_7))
  (bind _returnvalue_11 (Math|Float|SelectFloat _returnvalue_9 _returnvalue_6 _returnvalue_10))
  (bind _returnvalue_12 (* _returnvalue_11 -1.0))
  ;[0 0.3961 0.03922] I yell at myself to comment -Mabel
  (Utilities|FlowControl|Gate true) ; enters at Close
)

(event EventBlueprintActivate
  (params (Duration :type Float%20%28single-precision%29))
  (bind _returnvalue (Class|BasePart|GetPartWorldLocation))
  (bind _self self)
  (bind _returnvalue_2 (Utilities|GetOuterObject _self))
  (bind _aspart_grid_component (Utilities|Casting|CastToPartGridComponent _returnvalue_2))
  (bind _returnvalue_3 (Class|PartGridComponent|GetPartGridBounds _aspart_grid_component))
  (bind _returnvalue_4 (Math|Conversions|ToVector2D(IntPoint) (.upperbounds _returnvalue_3)))
  (bind _returnvalue_5 (Math|Conversions|ToVector2D(IntPoint) (.lowerbounds _returnvalue_3)))
  (bind _returnvalue_6 (Math|Vector2D|Vector2DLength _returnvalue_4))
  (bind _returnvalue_7 (Class|KismetMathLibrary|VSize2DSquared _returnvalue_4))
  (bind _returnvalue_8 (Class|KismetMathLibrary|VSize2DSquared _returnvalue_5))
  (bind _returnvalue_9 (Math|Vector2D|Vector2DLength _returnvalue_5))
  (bind _returnvalue_10 (> _returnvalue_8 _returnvalue_7))
  (bind _returnvalue_11 (Math|Float|SelectFloat _returnvalue_9 _returnvalue_6 _returnvalue_10))
  (bind _returnvalue_12 (* _returnvalue_11 -1.0))
  ;[0 0.3961 0.03922] I yell at myself to comment -Mabel
  (Utilities|FlowControl|Gate true) ; enters at Open
)

(event EventOnTick
  (params (DeltaTime :type Float%20%28single-precision%29))
  (bind _returnvalue (Class|BasePart|GetPartWorldLocation))
  (bind _self self)
  (bind _returnvalue_2 (Utilities|GetOuterObject _self))
  (bind _aspart_grid_component (Utilities|Casting|CastToPartGridComponent _returnvalue_2))
  (bind _returnvalue_3 (Class|PartGridComponent|GetPartGridBounds _aspart_grid_component))
  (bind _returnvalue_4 (Math|Conversions|ToVector2D(IntPoint) (.upperbounds _returnvalue_3)))
  (bind _returnvalue_5 (Math|Conversions|ToVector2D(IntPoint) (.lowerbounds _returnvalue_3)))
  (bind _returnvalue_6 (Math|Vector2D|Vector2DLength _returnvalue_4))
  (bind _returnvalue_7 (Class|KismetMathLibrary|VSize2DSquared _returnvalue_4))
  (bind _returnvalue_8 (Class|KismetMathLibrary|VSize2DSquared _returnvalue_5))
  (bind _returnvalue_9 (Math|Vector2D|Vector2DLength _returnvalue_5))
  (bind _returnvalue_10 (> _returnvalue_8 _returnvalue_7))
  (bind _returnvalue_11 (Math|Float|SelectFloat _returnvalue_9 _returnvalue_6 _returnvalue_10))
  (bind _returnvalue_12 (* _returnvalue_11 -1.0))
  ;[0 0.3961 0.03922] I yell at myself to comment -Mabel
  (Utilities|FlowControl|Gate true
    (:Exit
      (bind (_outactors _returnvalue_13) (Collision|SphereOverlapActors _returnvalue _returnvalue_11 (Utilities|Array|MakeArray "ObjectTypeQuery3" "ObjectTypeQuery1" "ObjectTypeQuery2") 0))
      (if _returnvalue_13
        (Rendering|Debug|DrawDebugSphere _returnvalue _returnvalue_11 12 "(R=1.000000,G=0.008275,B=0.000000,A=1.000000)" 1234.0 1.0)
        (Variables|Default|SetCheckX _returnvalue_12)
        (Variables|Default|SetCheckY _returnvalue_12)
        (while (>= _returnvalue_11 (Variables|Default|GetCheckY))
          (for _array_element _outactors
            (Development|PrintString "Hello")
            ;;[1 0 0] This needs to be fixed - Liam Suggestion
            (Variables|Default|SetCheckGridLocation (Utilities|Struct|MakeIntPoint (Math|Float|Round (+ (Variables|Default|GetCheckX) (.x (+ (Math|Transform|InverseTransformLocation (Transformation|GetActorTransform _array_element) (Class|BasePart|GetPartWorldLocation)) (Class|ShipPhysicsComponent|GetCenterOfMass (Variables|/Script/Voidsinger.BaseShip|GetPhysicsComponent (.AsBase%20Ship (Utilities|Casting|CastToBaseShip _array_element)))))))) (Math|Float|Round (+ (.y (+ (Math|Transform|InverseTransformLocation (Transformation|GetActorTransform _array_element) (Class|BasePart|GetPartWorldLocation)) (Class|ShipPhysicsComponent|GetCenterOfMass (Variables|/Script/Voidsinger.BaseShip|GetPhysicsComponent (.AsBase%20Ship (Utilities|Casting|CastToBaseShip _array_element)))))) (Variables|Default|GetCheckY))))))
          (bind _result (Math|Float|IncrementFloat (Variables|Default|GetCheckX))
            (:%20%20
              (if (> _result _returnvalue_11)
                (Math|Float|IncrementFloat (Variables|Default|GetCheckY)
                  (:%20%20
                    (Variables|Default|SetCheckX (* _returnvalue_11 -1.0))))))))))))

(event EventBeginPlay
  ;[0 0.3961 0.03922] I yell at myself to comment -Mabel
  (EventDispatchers|BindEventtoOnDeactivateVoidsongDelegate (CallFunction|GetStarSystemGameMode) (delegate Custom|Deactivate)))

(event EventOnCriticallyDamaged
  (bind _returnvalue (Class|BasePart|GetShip))
  (bind _asstarsystemplayerstate (CallFunction|GetStarSystemPlayerState))
  (switch Utilities|FlowControl|Switch|SwitchonEFactions (Class|BaseShip|GetFaction _returnvalue)
    (:Player
      (Default|CallOnPlayerDeath (CallFunction|GetStarSystemGameMode)))
    (:Enemy
      (Class|ShipPlayerState|DepositPixels _asstarsystemplayerstate (Math|Float|Round (* (Variables|/Script/Voidsinger.BaseShip|GetPixelValue _returnvalue) (Variables|/Script/Voidsinger.ShipPlayerState|GetPixelHarvestingEfficiency _asstarsystemplayerstate))))
      ;[0.2986 0.2986 0.2986] Add fuel when an enemy dies for each fuel system
      (for _array_element (Class|BaseShip|GetResourceSystems (.AsPlayer%20Ship (Utilities|Casting|CastToPlayerShip (Game|Player|GetPlayerPawn 0))))
        (if (Utilities|Enum|Equal(Enum) (Class|BaseResourceSystem|GetType _array_element) "Fuel")
          (Class|BaseResourceSystem|AddResources _array_element 1e+02))))))