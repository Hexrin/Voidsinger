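; BP_Hull is a hull part Blueprint that currently only reports its lifecycle and damage states as debug messages.
; Its destroyed, critically damaged, damaged, BeginPlay and tick events each print the part's display name with a state label, color-coded per event.
; The PartFunctionDebug flag from the DebugSettings class defaults gates both screen and log output; no hull gameplay logic runs in this graph.
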(event EventBeginPlay
  (bind _partfunctiondebug (Utilities|GetClassDefaults "/Game/DebugSettings.DebugSettings_C"))
  ;[0 0.3961 0.03922] Comment this
  (Development|PrintString (Utilities|String|Append (Utilities|GetDisplayName self) ": BeginPlay") _partfunctiondebug _partfunctiondebug "(R=0.000000,G=1.000000,B=0.064159,A=1.000000)" 6e+01))

(event EventEventDamaged
  (bind _partfunctiondebug (Utilities|GetClassDefaults "/Game/DebugSettings.DebugSettings_C"))
  ;[0 0.3961 0.03922] Comment this
  (Development|PrintString (Utilities|String|Append (Utilities|GetDisplayName self) ": Damaged") _partfunctiondebug _partfunctiondebug "(R=0.814109,G=1.000000,B=0.000000,A=1.000000)" 1e+01))

(event EventEventDestroyed
  (bind _partfunctiondebug (Utilities|GetClassDefaults "/Game/DebugSettings.DebugSettings_C"))
  ;[0 0.3961 0.03922] Comment this
  (Development|PrintString (Utilities|String|Append (Utilities|GetDisplayName self) ": Destroyed") _partfunctiondebug _partfunctiondebug "(R=1.000000,G=0.751714,B=0.000000,A=1.000000)" 6e+01))

(event EventOnTick
  (params (DeltaTime :type Float%20%28single-precision%29))
  (bind _partfunctiondebug (Utilities|GetClassDefaults "/Game/DebugSettings.DebugSettings_C"))
  ;[0 0.3961 0.03922] Comment this
  (Development|PrintString (Utilities|String|Append (Utilities|GetDisplayName self) ": Tick     |     Delta Seconds: " (Utilities|String|ToString(Float) DeltaTime)) _partfunctiondebug _partfunctiondebug "(R=0.000000,G=0.208848,B=1.000000,A=1.000000)" 0.1))

(event EventEventCriticalyDamaged
  (bind _partfunctiondebug (Utilities|GetClassDefaults "/Game/DebugSettings.DebugSettings_C"))
  ;[0 0.3961 0.03922] Comment this
  (Development|PrintString (Utilities|String|Append (Utilities|GetDisplayName self) ": Criticaly Damaged") _partfunctiondebug _partfunctiondebug "(R=1.000000,G=0.945338,B=0.000000,A=1.000000)" 2e+01))