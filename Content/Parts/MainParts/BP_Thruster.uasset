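; Thruster part on a part grid; this Blueprint only adds a debug visualization of its thrust on tick.
; When MovementDebug is on in DebugSettings, it rotates the thrust location and direction by the grid owner's yaw in 2D to place a world-space arrow.
; The dark blue arrow ends at the thrust point, with length scaled by thrust force.
; While thrusting, a thicker red arrow is drawn over it.
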(event EventOnTick
  (params (DeltaTime :type Float%20%28single-precision%29))
  (bind _returnvalue (Class|BaseThrusterPart|GetThrustRotation))
  (bind _returnvalue_2 (Class|BaseThrusterPart|GetThrustRelativeLocation))
  (bind _returnvalue_3 (Class|BasePart|GetPartGrid))
  (bind _returnvalue_4 (Class|BaseThrusterPart|GetThrustForce))
  (bind _returnvalue_5 (Components|GetOwner _returnvalue_3))
  (bind _returnvalue_6 (* _returnvalue_4 -0.1))
  (bind _returnvalue_7 (Transformation|GetActorLocation _returnvalue_5))
  (bind _returnvalue_8 (Transformation|GetActorRotation _returnvalue_5))
  (bind _returnvalue_9 (Class|KismetMathLibrary|GetRotated2D _returnvalue_2 (.yaw _returnvalue_8)))
  (bind _returnvalue_10 (+ (.yaw _returnvalue_8) _returnvalue))
  (bind _returnvalue_11 (Class|KismetMathLibrary|GetRotated2D (Math|Vector2D|MakeVector2D _returnvalue_6 0.0) _returnvalue_10))
  (bind _returnvalue_12 (+ _returnvalue_7 _returnvalue_9))
  (bind _returnvalue_13 (+ _returnvalue_12 _returnvalue_11))
  (if (.MovementDebug (Utilities|GetClassDefaults "/Game/DebugSettings.DebugSettings_C"))
    (Rendering|Debug|DrawDebugArrow _returnvalue_13 _returnvalue_12 0.25 "(R=0.000000,G=0.030755,B=0.324653,A=1.000000)" 0.0 0.1)
    (if (Class|BaseThrusterPart|IsThrusting)
      (Rendering|Debug|DrawDebugArrow _returnvalue_13 _returnvalue_12 0.5 "(R=1.000000,G=0.000000,B=0.000000,A=1.000000)" 0.0 0.2))))