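; BP_Thruster is a thruster ship part whose graph handles debug visualization of thrust.
; When MovementDebug is on, tick draws an arrow at the thrust point, rotated by ship yaw and offset from the center of mass, sized by thrust force.
; While thrusting, a throttle-scaled counter accumulates and counts down in a loop that spawns nothing.
; The ThrusterGas spawn logic, with random arc and point velocity, is disconnected.
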(event EventOnTick
  (params (DeltaTime :type Float%20%28single-precision%29))
  (bind _returnvalue (Class|BasePart|GetShip))
  (bind _returnvalue_2 (Class|BaseThrusterPart|GetThrustRelativeLocation))
  (bind _returnvalue_3 (Class|BasePart|GetPartGrid))
  (bind _returnvalue_4 (Transformation|GetActorLocation _returnvalue))
  (bind _returnvalue_5 (Components|GetOwner _returnvalue_3))
  (bind _physicscomponent (Variables|/Script/Voidsinger.BaseShip|GetPhysicsComponent _returnvalue))
  (bind _returnvalue_6 (Class|ShipPhysicsComponent|GetCenterOfMass _physicscomponent))
  (bind _returnvalue_7 (Transformation|GetActorRotation _returnvalue_5))
  (bind _returnvalue_8 (Class|KismetMathLibrary|GetRotated2D _returnvalue_2 (.yaw _returnvalue_7)))
  (bind _returnvalue_9 (- _returnvalue_4 _returnvalue_6))
  (bind _returnvalue_10 (+ _returnvalue_8 _returnvalue_9))
  (if (.MovementDebug (Utilities|GetClassDefaults "/Game/DebugSettings.DebugSettings_C"))
    (Rendering|Debug|DrawDebugArrow (+ _returnvalue_10 (Class|KismetMathLibrary|GetRotated2D (Math|Vector2D|MakeVector2D (* (Class|BaseThrusterPart|GetThrustForce) -0.1) 0.0) (+ (.yaw _returnvalue_7) (Class|BaseThrusterPart|GetThrustRotation)))) _returnvalue_10 0.25 "(R=0.000000,G=0.030755,B=0.324653,A=1.000000)" 0.0 0.1)
    (if (Class|BaseThrusterPart|IsThrusting)
      (bind _output_get (Variables|Default|SetCountyBoi (+ (Variables|Default|GetCountyBoi) (* (Class|BaseThrusterPart|GetThrottle) (Variables|Default|GetFrequencyBoi) DeltaTime))))
      (for _index (range 0 (Math|Float|Truncate _output_get))
        (Math|Float|DecrementFloat _output_get)))))