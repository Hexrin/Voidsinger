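; Cluster cannon ship part that spawns a projectile with a given explosion radius and velocity, passing along the ship's velocity.
; On tick it binds its fire event to the player ship's cannon binding, while activation calls Cannon with preset radius and velocity.
; Firing has no live ammo check, as the condition is always true.
; Ammo and muzzle-offset logic is left unreachable or unused, and NewFunction_0 is empty.
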(event Custom|CustomEvent
  (params (Radius :type Float%20%28single-precision%29) (Velocity :type Float%20%28single-precision%29))
  (if true
    (Game|SpawnActorfromClass "/Game/Parts/MainParts/CannonParts/Projectile.Projectile_C" (Math|Transform|MakeTransform "0, 0, 0" "0, 0, 0" "1,1,1") "AlwaysSpawn" 0 Radius Velocity (Math|Conversions|ToVector(Vector2D) (Class|ShipPhysicsComponent|GetVelocity (Variables|/Script/Voidsinger.BaseShip|GetPhysicsComponent (Class|BasePart|GetShip)))) 0.0 0 0)))

(event EventBlueprintActivate
  (CallFunction|Cannon 1.3 0.6))

(event EventOnTick
  (params (DeltaTime :type Float%20%28single-precision%29))
  (bind _asbp_player_ship (Utilities|Casting|CastToBP_PlayerShip (Class|BasePart|GetShip)))
  (EventDispatchers|BindEventtoCannon _asbp_player_ship (delegate Custom|CustomEvent)))

(fn NewFunction0)