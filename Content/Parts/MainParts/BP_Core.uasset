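; Ship core part that, while activated, applies effects to nearby actors and shows a demo death screen when critically damaged on the player's ship.
; A Gate opened on activation and closed by the game mode's Voidsong deactivate delegate runs a per-tick sphere overlap sized from the part grid bounds.
; It sweeps grid cells across that radius, calling ActivateWithEffects scaled by DeltaTime.
; The sweep is unfinished, with debug drawing, prints and an always-true hit check.
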(event Custom|Deactivate
  (bind _returnvalue (Class|BasePart|GetPartWorldLocation))
  (bind _self self)
  (bind _returnvalue_2 (Utilities|GetOuterObject _self))
  (bind _returnvalue_3 (Utilities|GetOuterObject _returnvalue_2))
  (bind _aspart_grid_component (Utilities|Casting|CastToPartGridComponent _returnvalue_2))
  (bind _returnvalue_4 (Class|PartGridComponent|GetPartGridBounds _aspart_grid_component))
  (bind _asactor (Utilities|Casting|CastToActor _returnvalue_3))
  (bind _returnvalue_5 (Math|Conversions|ToVector2D(IntPoint) (.upperbounds _returnvalue_4)))
  (bind _returnvalue_6 (Math|Conversions|ToVector2D(IntPoint) (.lowerbounds _returnvalue_4)))
  (bind _returnvalue_7 (Math|Vector2D|Vector2DLength _returnvalue_5))
  (bind _returnvalue_8 (Class|KismetMathLibrary|VSize2DSquared _returnvalue_5))
  (bind _returnvalue_9 (Class|KismetMathLibrary|VSize2DSquared _returnvalue_6))
  (bind _returnvalue_10 (Math|Vector2D|Vector2DLength _returnvalue_6))
  (bind _returnvalue_11 (> _returnvalue_9 _returnvalue_8))
  (bind _returnvalue_12 (Math|Float|SelectFloat _returnvalue_10 _returnvalue_7 _returnvalue_11))
  (bind _returnvalue_13 (* _returnvalue_12 -1.0))
  (Utilities|FlowControl|Gate true) ; enters at Close
)

(event EventBlueprintActivate
  (bind _returnvalue (Class|BasePart|GetPartWorldLocation))
  (bind _self self)
  (bind _returnvalue_2 (Utilities|GetOuterObject _self))
  (bind _returnvalue_3 (Utilities|GetOuterObject _returnvalue_2))
  (bind _aspart_grid_component (Utilities|Casting|CastToPartGridComponent _returnvalue_2))
  (bind _returnvalue_4 (Class|PartGridComponent|GetPartGridBounds _aspart_grid_component))
  (bind _asactor (Utilities|Casting|CastToActor _returnvalue_3))
  (bind _returnvalue_5 (Math|Conversions|ToVector2D(IntPoint) (.upperbounds _returnvalue_4)))
  (bind _returnvalue_6 (Math|Conversions|ToVector2D(IntPoint) (.lowerbounds _returnvalue_4)))
  (bind _returnvalue_7 (Math|Vector2D|Vector2DLength _returnvalue_5))
  (bind _returnvalue_8 (Class|KismetMathLibrary|VSize2DSquared _returnvalue_5))
  (bind _returnvalue_9 (Class|KismetMathLibrary|VSize2DSquared _returnvalue_6))
  (bind _returnvalue_10 (Math|Vector2D|Vector2DLength _returnvalue_6))
  (bind _returnvalue_11 (> _returnvalue_9 _returnvalue_8))
  (bind _returnvalue_12 (Math|Float|SelectFloat _returnvalue_10 _returnvalue_7 _returnvalue_11))
  (bind _returnvalue_13 (* _returnvalue_12 -1.0))
  (Utilities|FlowControl|Gate true) ; enters at Open
)

(event EventOnTick
  (params (DeltaTime :type Float%20%28single-precision%29))
  (bind _returnvalue (Class|BasePart|GetPartWorldLocation))
  (bind _self self)
  (bind _returnvalue_2 (Utilities|GetOuterObject _self))
  (bind _returnvalue_3 (Utilities|GetOuterObject _returnvalue_2))
  (bind _aspart_grid_component (Utilities|Casting|CastToPartGridComponent _returnvalue_2))
  (bind _returnvalue_4 (Class|PartGridComponent|GetPartGridBounds _aspart_grid_component))
  (bind _asactor (Utilities|Casting|CastToActor _returnvalue_3))
  (bind _returnvalue_5 (Math|Conversions|ToVector2D(IntPoint) (.upperbounds _returnvalue_4)))
  (bind _returnvalue_6 (Math|Conversions|ToVector2D(IntPoint) (.lowerbounds _returnvalue_4)))
  (bind _returnvalue_7 (Math|Vector2D|Vector2DLength _returnvalue_5))
  (bind _returnvalue_8 (Class|KismetMathLibrary|VSize2DSquared _returnvalue_5))
  (bind _returnvalue_9 (Class|KismetMathLibrary|VSize2DSquared _returnvalue_6))
  (bind _returnvalue_10 (Math|Vector2D|Vector2DLength _returnvalue_6))
  (bind _returnvalue_11 (> _returnvalue_9 _returnvalue_8))
  (bind _returnvalue_12 (Math|Float|SelectFloat _returnvalue_10 _returnvalue_7 _returnvalue_11))
  (bind _returnvalue_13 (* _returnvalue_12 -1.0))
  (Utilities|FlowControl|Gate true
    (:Exit
      (bind (_outactors _returnvalue_14) (Collision|SphereOverlapActors _returnvalue _returnvalue_12 (Utilities|Array|MakeArray "ObjectTypeQuery3" "ObjectTypeQuery1" "ObjectTypeQuery2") 0))
      (if _returnvalue_14
        (Rendering|Debug|DrawDebugSphere _returnvalue _returnvalue_12 12 "(R=1.000000,G=0.008275,B=0.000000,A=1.000000)" 1234.0 1.0)
        (Variables|Default|SetCheckX _returnvalue_13)
        (Variables|Default|SetCheckY _returnvalue_13)
        (while (>= _returnvalue_12 (Variables|Default|GetCheckY))
          (for _array_element _outactors
            (Development|PrintString "Hello")
            (Variables|Default|SetCheckGridLocation (Utilities|Struct|MakeIntPoint (Math|Float|Round (+ (Variables|Default|GetCheckX) (.x (+ (Math|Transform|InverseTransformLocation (Transformation|GetActorTransform _array_element) (Class|BasePart|GetPartWorldLocation)) (Class|ShipPhysicsComponent|GetCenterOfMass (Variables|/Script/Voidsinger.BaseShip|GetPhysicsComponent (.AsBase%20Ship (Utilities|Casting|CastToBaseShip _array_element)))))))) (Math|Float|Round (+ (.y (+ (Math|Transform|InverseTransformLocation (Transformation|GetActorTransform _array_element) (Class|BasePart|GetPartWorldLocation)) (Class|ShipPhysicsComponent|GetCenterOfMass (Variables|/Script/Voidsinger.BaseShip|GetPhysicsComponent (.AsBase%20Ship (Utilities|Casting|CastToBaseShip _array_element)))))) (Variables|Default|GetCheckY)))))
            (if true
              (Development|PrintString "Hello")
              (Class|VoidGameMode|ActivatewithEffects (.AsVoid%20Game%20Mode (Utilities|Casting|CastToVoidGameMode (Game|GetGameMode))) _array_element _asactor (Utilities|Array|MakeArray 0) (Class|BasePart|GetPartWorldLocation) (Math|Transform|TransformLocation (Transformation|GetActorTransform _asactor) (Math|Conversions|ToVector(Vector2D) (- (Variables|Default|GetCheckGridLocation) (Class|ShipPhysicsComponent|GetCenterOfMass (Variables|/Script/Voidsinger.BaseShip|GetPhysicsComponent (.AsBase%20Ship (Utilities|Casting|CastToBaseShip _array_element))))))) DeltaTime)
              (else
                (Development|PrintString "Hello"))))
          (bind _result (Math|Float|IncrementFloat (Variables|Default|GetCheckX))
            (:%20%20
              (if (> _result _returnvalue_12)
                (Math|Float|IncrementFloat (Variables|Default|GetCheckY)
                  (:%20%20
                    (Variables|Default|SetCheckX (* _returnvalue_12 -1.0))))))))))))

(event EventBeginPlay
  (EventDispatchers|BindEventtoOnDeactivateVoidsongDelegate (.AsVoid%20Game%20Mode (Utilities|Casting|CastToVoidGameMode (Game|GetGameMode))) (delegate Custom|Deactivate)))

(event EventOnCriticallyDamaged
  ;[1 1 1] fully aware this is ehhhh but demo stuff, y'know? Probably will want to have a death function on the base ship rather than this.
  (if (== (Game|Player|GetPlayerPawn 0) (Utilities|GetOuterObject (Utilities|GetOuterObject self)))
    (bind _returnvalue (UserInterface|CreateWidget "/Game/UI/MainMenuUI/YouDiedDemo.YouDiedDemo_C"))
    (UserInterface|Viewport|AddtoViewport _returnvalue 0)))