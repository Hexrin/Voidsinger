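; BP_GigaLaser is a laser ship part that box-traces along a segment and applies heat to the hit BaseShip's part grid.
; If the hit part implements I_LaserInterface, it returns new segments, each applying heat at the hit and recursively firing another laser.
; Otherwise the beam ends, applying damage-scaled heat without delta-time scaling, printing the value and activating Voidsongs on the hit actor.
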(fn FireLaser
  (params (StartEndLocation :type S%20Start%20End%20Data%20Structure))
  (bind _damage (Variables|Default|GetDamage))
  (bind _returnvalue (* _damage (.damage StartEndLocation)))
  (bind _outhit (Collision|BoxTraceByChannel (.startlocation StartEndLocation) (.endlocation StartEndLocation) (Variables|Default|GetHalf%20Size) "0, 0, 0" "TraceTypeQuery1" false 0 "None"))
  (bind _asbase_ship (Utilities|Casting|CastToBaseShip (.HitActor (Collision|BreakHitResult _outhit))))
  (if (Utilities|DoesObjectImplementInterface (Utilities|Array|Get(acopy) (Class|FunctionLibrary|GetPartsHitfromWorldLocation (.Location (Collision|BreakHitResult _outhit)) (Variables|/Script/Voidsinger.BaseShip|GetPartGrid _asbase_ship))) "/Game/Parts/Lasers/LaserRedirectors/I_LaserInterface.I_LaserInterface_C")
    (bind _laserresults (Class|ILaserInterface|LaserData(Message) (Utilities|Array|Get(acopy) (Class|FunctionLibrary|GetPartsHitfromWorldLocation (.Location (Collision|BreakHitResult _outhit)) (Variables|/Script/Voidsinger.BaseShip|GetPartGrid _asbase_ship))) _outhit (Variables|Default|GetDistanceTraveled) (.damage StartEndLocation)))
    (for _array_element _laserresults
      (Class|PartGridComponent|ApplyHeatatLocation (Variables|/Script/Voidsinger.BaseShip|GetPartGrid _asbase_ship) (.Location (Collision|BreakHitResult _outhit)) (* (Variables|Default|GetDamage) (.damage _array_element)))
      (CallFunction|FireLaser (Utilities|Struct|MakeS_StartEndData (.startlocation _array_element) (.endlocation _array_element) 0.0 (.damage _array_element))))
    (else
      ;[1 1 1] Damade not multiplied by delta seconds
      (Class|PartGridComponent|ApplyHeatatLocation (Variables|/Script/Voidsinger.BaseShip|GetPartGrid _asbase_ship) (.Location (Collision|BreakHitResult _outhit)) _returnvalue)
      (Development|PrintString (Utilities|String|ToString(Float) _returnvalue))
      (CallFunction|ActivateVoidsongs (.HitActor (Collision|BreakHitResult _outhit))))))