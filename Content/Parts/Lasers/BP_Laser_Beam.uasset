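; Short-lived laser beam actor that draws a plane between a start point and an end point.
; The construction script sets the plane's width, turns the root toward the end point and stretches it along X by the 2D distance between the points.
; On Tick, an initially closed DoOnce that is reset each frame skips the first tick and destroys the actor on the next.
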(event EventTick
  (params (DeltaSeconds :type Float%20%28single-precision%29))
  (Utilities|FlowControl|Sequence
    (:then_0
      (Utilities|FlowControl|DoOnce true :!label _label
        (:Completed
          (Actor|DestroyActor))))
    (:then_1
      (goto _label Reset))))

(fn ConstructionScript
  (bind _startpoint (Variables|Default|GetStartPoint))
  (bind _endpoint (Variables|Default|GetEndPoint))
  (bind _root (Variables|Default|GetRoot))
  (Transformation|SetRelativeScale3D (Variables|Default|GetPlane) (Math|Vector|MakeVector 1.0 (Variables|Default|GetWidth) 1.0))
  (Transformation|SetWorldRotation _root (Math|Rotator|FindLookatRotation _startpoint _endpoint) false false)
  (Transformation|SetWorldScale3D _root (Math|Vector|MakeVector (Math|Vector|Distance2D(Vector) _startpoint _endpoint) 1.0 1.0)))