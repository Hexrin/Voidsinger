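; BP_LaserCombiner is a ship laser redirector part that computes the outgoing beam for a laser that hits it.
; LaserData places the beam start at the rotated combiner offset on the hit ship, using 2D yaw rotation.
; The beam follows ship forward turned by part rotation, for the passed distance minus hit distance, with damage scaled by PercentDispatched.
; ReflectionEfficiency reports the absorbed and dispatched fractions.
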(fn LaserData
  (params (DataInput :type Hit%20Result%20Structure) (DistanceTraveled :type Float%20%28single-precision%29) (Damage :type Float%20%28single-precision%29))
  (bind _returnvalue (Class|BasePart|GetPartRelativeLocation))
  (bind _returnvalue_2 (Class|BasePart|GetRelativeRotation))
  (bind _returnvalue_3 (Transformation|GetActorLocation (.hitactor DataInput)))
  (bind _returnvalue_4 (Transformation|GetActorRotation (.hitactor DataInput)))
  (bind _asbase_ship (Utilities|Casting|CastToBaseShip (.hitactor DataInput)))
  (bind _combineroffset (Variables|Default|GetCombinerOffset))
  (bind _returnvalue_5 (Class|KismetMathLibrary|GetRotated2D _combineroffset _returnvalue_2))
  (bind _physicscomponent (Variables|/Script/Voidsinger.BaseShip|GetPhysicsComponent _asbase_ship))
  (bind _returnvalue_6 (Class|ShipPhysicsComponent|GetCenterOfMass _physicscomponent))
  (bind _returnvalue_7 (+ _returnvalue _returnvalue_5))
  (bind _returnvalue_8 (Math|Conversions|ToVector2D(Vector) _returnvalue_7))
  (bind _returnvalue_9 (+ _returnvalue_3 _returnvalue_6))
  (bind _returnvalue_10 (Class|KismetMathLibrary|GetRotated2D _returnvalue_8 (.yaw _returnvalue_4)))
  (bind _returnvalue_11 (+ _returnvalue_9 _returnvalue_10))
  (bind _returnvalue_12 (- _returnvalue_11 _returnvalue_6))
  (return (Utilities|Array|MakeArray (Utilities|Struct|MakeS_StartEndData _returnvalue_12 (+ _returnvalue_12 (Math|Vector|RotateVector (* (Transformation|GetActorForwardVector (.hitactor DataInput)) (- DistanceTraveled (.distance DataInput))) (Math|Rotator|MakeRotator 0.0 0.0 (Class|BasePart|GetRelativeRotation)))) 0.0 (* Damage (Variables|Default|GetPercentDispatched))))))

(fn ReflectionEfficiency
  (return (Variables|Default|GetPercentAbsorbed) (Variables|Default|GetPercentDispatched)))