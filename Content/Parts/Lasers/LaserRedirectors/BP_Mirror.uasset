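; BP_Mirror is a laser redirector part that bounces an incoming laser off its surface.
; Laser Data mirrors the beam about the impact normal, offsets the origin slightly off the surface, passes on the remaining length and scales effectiveness by the reflected percentage.
; Hits that begin inside the mirror are skipped to prevent infinite loops.
; ReflectionEfficiency reports absorbed and reflected shares, and EdGraph_26 holds a similar reflection calculation.
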(fn EdGraph26
  (params (DataInput :type Hit%20Result%20Structure) (DistanceTraveled :type Float%20%28single-precision%29))
  (return (Utilities|Array|MakeArray (Utilities|Struct|MakeS_LaserInformation (+ (.location DataInput) (* (.normal DataInput) 0.01)) "0.000000,0.000000,0.000000" 0.0 0.0 (* (- DistanceTraveled (.distance DataInput)) (Math|Vector|MirrorVectorbyNormal (Math|Vector|Normalize (- (.traceend DataInput) (.tracestart DataInput))) (.normal DataInput)))))))

(fn LaserData
  (params (LaserHit :type Hit%20Result%20Structure) (LaserInfo :type S%20Laser%20Information%20Structure))
  (bind (_bblockinghit _binitialoverlap _time _distance _location _impactpoint _normal _impactnormal _physmat _hitactor _hitcomponent _hitbonename _hititem _elementindex _faceindex _tracestart _traceend) (Collision|BreakHitResult LaserHit))
  (if (not _binitialoverlap) ; Prevent infinite loops caused by lasers being stuck inside a mirror
    (return (Utilities|Array|MakeArray (Utilities|Struct|MakeS_LaserInformation (+ _location (* _impactnormal 0.01)) (Math|Vector|MirrorVectorbyNormal (Math|Vector|GetUnitDirection(Vector) _tracestart _traceend) _impactnormal) (* (.laserlength LaserInfo) (- 1.0 _time)) (* (.effectiveness LaserInfo) (Variables|Default|GetPercentReflected)))))))

(fn ReflectionEfficiency
  (return (Variables|Default|GetPercentAbsorbed) (Variables|Default|GetPercentReflected)))