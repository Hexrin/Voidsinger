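; BP_LaserBeam is a short-lived actor that shows a laser beam as a plane stretched between a start and end point.
; Its construction script sets the plane's width, scales the actor by the 2D distance between the points, and rotates it from the start toward the end.
; On Tick, a DoOnce that appears to start closed is reset after each check, so the beam destroys itself on its second tick.
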(event EventTick
  (params (DeltaSeconds :type Float%20%28single-precision%29))
  (Utilities|FlowControl|Sequence
    (:then_0
      (Utilities|FlowControl|DoOnce true :!label _label
        (:Completed
          (Actor|DestroyActor))))
    (:then_1
      (goto _label Reset))))

(fn ConstructionScript
  (bind _startpoint (Variables|Default|GetStartPoint))
  (Transformation|SetRelativeScale3D (Variables|Default|GetPlane) (Math|Vector|MakeVector 1.0 (Variables|Default|GetWidth) 1.0))
  (Transformation|SetActorScale3D (Math|Vector|MakeVector (Math|Vector|Distance2D(Vector) (Variables|Default|GetStartPoint) (Variables|Default|GetEndPoint)) 1.0 1.0))
  (Transformation|SetActorLocationAndRotation _startpoint (Math|Rotator|FindLookatRotation _startpoint (Variables|Default|GetEndPoint))))