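; Laser ship part that, after a charge-up effect and delay, fires a beam for the activation duration.
; Each tick it draws electricity to fire, flickering while power is short.
; FireLaser line-traces, spawns a velocity-compensated beam and recursively fires new beams returned by hit parts implementing I_LaserInterface.
; Ship hits spawn an impact effect, apply absorption-scaled heat to the part grid and report to the star system level manager.
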(event EventOnTick
  (params (DeltaTime :type Float%20%28single-precision%29))
  (bind _returnvalue (Class|BasePart|GetShip))
  (bind _physicscomponent (Variables|/Script/Voidsinger.BaseShip|GetPhysicsComponent _returnvalue))
  (bind _returnvalue_2 (Class|ShipPhysicsComponent|GetCenterOfMass _physicscomponent))
  (Utilities|FlowControl|Gate true :!label _label
    (:Exit
      (bind _returnvalue_3 (Class|BaseResourceSystem|DrawResources (Class|BasePart|GetSystembyType "Electricity") (* DeltaTime (Variables|Default|GetElectricityUsageRate))))
      (if _returnvalue_3
        (CallFunction|FireLaser (Utilities|Struct|MakeS_LaserInformation (- (+ (+ (Transformation|GetActorLocation _returnvalue) _returnvalue_2) (Class|KismetMathLibrary|GetRotated2D (Math|Conversions|ToVector2D(Vector) (+ (Class|BasePart|GetPartRelativeLocation) (Class|KismetMathLibrary|GetRotated2D (Variables|Default|GetLaserStartLocation) (Class|BasePart|GetRelativeRotation)))) (.yaw (Transformation|GetActorRotation _returnvalue)))) _returnvalue_2) (Math|Vector|RotateVector (Transformation|GetActorForwardVector (Class|BasePart|GetShip)) (Math|Rotator|MakeRotator 0.0 0.0 (Class|BasePart|GetRelativeRotation))) (Variables|Default|GetLaserLength) 1.0) (stale EventBlueprintActivate Duration))
        (else
          ;[1 1 1] Flicker slower when out of resouceses
          (Utilities|FlowControl|Sequence
            (:then_0
              (Utilities|FlowControl|Delay 0.5)
              (Utilities|FlowControl|Gate true
                (:Exit
                  (goto _label Open))))
            (:then_1
              (goto _label Close))))))))

(event EventBlueprintActivate
  (params (Duration :type Float%20%28single-precision%29))
  (bind _returnvalue (Class|BasePart|GetPartRelativeLocation))
  (bind _returnvalue_2 (Class|BasePart|GetShip))
  (bind _returnvalue_3 (Class|BasePart|GetRelativeRotation))
  (bind _laserstartlocation (Variables|Default|GetLaserStartLocation))
  (bind _returnvalue_4 (Class|KismetMathLibrary|GetRotated2D _laserstartlocation _returnvalue_3))
  (bind _returnvalue_5 (Transformation|GetActorLocation _returnvalue_2))
  (bind _returnvalue_6 (Transformation|GetActorRotation _returnvalue_2))
  (bind _physicscomponent (Variables|/Script/Voidsinger.BaseShip|GetPhysicsComponent _returnvalue_2))
  (bind _returnvalue_7 (Class|ShipPhysicsComponent|GetCenterOfMass _physicscomponent))
  (bind _returnvalue_8 (+ _returnvalue _returnvalue_4))
  (bind _returnvalue_9 (Math|Conversions|ToVector2D(Vector) _returnvalue_8))
  (bind _returnvalue_10 (+ _returnvalue_5 _returnvalue_7))
  (bind _returnvalue_11 (Class|KismetMathLibrary|GetRotated2D _returnvalue_9 (.yaw _returnvalue_6)))
  (bind _returnvalue_12 (+ _returnvalue_10 _returnvalue_11))
  (bind _returnvalue_13 (- _returnvalue_12 _returnvalue_7))
  (bind _returnvalue_14 (Niagara|SpawnSystematLocation "/Game/FX/Systems/NS_LaserChargeUp.NS_LaserChargeUp" _returnvalue_13))
  (Niagara|SetNiagaraVariable(Float) _returnvalue_14 "Age" (Variables|Default|GetDelay))
  (bind _output_get (Variables|Default|SetDelay (Variables|Default|GetDelay)))
  (Utilities|FlowControl|Delay _output_get)
  (Utilities|FlowControl|Sequence
    (:then_0
      (Utilities|FlowControl|Gate true) ; enters at Open
    )
    (:then_1
      ;[1 1 1] Flicker slower when out of resouceses
      (Utilities|FlowControl|Gate true) ; enters at Open
    )
    (:then_2
      (Utilities|FlowControl|RetriggerableDelay Duration)
      (Utilities|FlowControl|Sequence
        (:then_0
          (Utilities|FlowControl|Gate true) ; enters at Close
        )
        (:then_1
          (Utilities|FlowControl|Gate true) ; enters at Close
        )))))

(fn FireLaser
  (params (LaserInfo :type S%20Laser%20Information%20Structure) (Duration :type Float%20%28single-precision%29))
  (bind _returnvalue (Class|BasePart|GetShip))
  (bind _returnvalue_2 (Utilities|Time|GetWorldDeltaSeconds))
  (bind _physicscomponent (Variables|/Script/Voidsinger.BaseShip|GetPhysicsComponent _returnvalue))
  (bind _returnvalue_3 (Class|ShipPhysicsComponent|GetVelocity _physicscomponent))
  (bind _returnvalue_4 (* _returnvalue_3 _returnvalue_2))
  (bind _outhit (CallFunction|TraceforLaser (.startlocation LaserInfo) (+ (.startlocation LaserInfo) (* (.firedirection LaserInfo) (.laserlength LaserInfo)))))
  (Game|SpawnActorfromClass "/Game/Parts/Lasers/BP_Laser_Beam.BP_Laser_Beam_C" (Math|Transform|MakeTransform (+ _returnvalue_4 (.startlocation LaserInfo)) "0, 0, 0" "1,1,1") "Undefined" 0 (+ _returnvalue_4 (select (.bBlockingHit (Collision|BreakHitResult _outhit)) (.Location (Collision|BreakHitResult _outhit)) (.TraceEnd (Collision|BreakHitResult _outhit)))) (Variables|Default|GetLaserWidth) Duration 0)
  (bind _asbase_ship (Utilities|Casting|CastToBaseShip (.HitActor (Collision|BreakHitResult _outhit))))
  (if (Utilities|DoesObjectImplementInterface (Utilities|Array|Get(acopy) (Class|FunctionLibrary|GetPartsHitfromWorldLocation (.ImpactPoint (Collision|BreakHitResult _outhit)) (Variables|/Script/Voidsinger.BaseShip|GetPartGrid _asbase_ship))) "/Game/Parts/Lasers/LaserRedirectors/I_LaserInterface.I_LaserInterface_C")
    (bind _newlaserstofire (Class|ILaserInterface|LaserData(Message) (Utilities|Array|Get(acopy) (Class|FunctionLibrary|GetPartsHitfromWorldLocation (.ImpactPoint (Collision|BreakHitResult _outhit)) (Variables|/Script/Voidsinger.BaseShip|GetPartGrid _asbase_ship))) _outhit LaserInfo))
    (CallFunction|ApplyHitEffect _outhit LaserInfo)
    (if (not (< (Math|Vector|DotProduct (.ImpactNormal (Collision|BreakHitResult _outhit)) (.firedirection LaserInfo)) 0.0))
      (for _array_element _newlaserstofire
        (CallFunction|FireLaser (Utilities|Struct|MakeS_LaserInformation (.startlocation _array_element) (.firedirection _array_element) (.laserlength _array_element) (.effectiveness _array_element)) 0.0)))
    (else
      (CallFunction|ApplyHitEffect _outhit LaserInfo))))

(fn TraceforLaser
  (params (Start :type Vector) (End :type Vector))
  (bind _outhit (Collision|LineTraceByChannel Start End "TraceTypeQuery1" false 0 "None" false "(R=0.350954,G=1.000000,B=0.000000,A=1.000000)" "(R=0.000000,G=0.000000,B=0.000000,A=0.000000)" 2.0))
  (return _outhit))

(fn ApplyHitEffect
  (params (LaserHit :type Hit%20Result%20Structure) (LaserInfo :type S%20Laser%20Information%20Structure))
  (bind (_bblockinghit _binitialoverlap _time _distance _location _impactpoint _normal _impactnormal _physmat _hitactor _hitcomponent _hitbonename _hititem _elementindex _faceindex _tracestart) (Collision|BreakHitResult LaserHit))
  (bind _returnvalue (Utilities|Time|GetWorldDeltaSeconds))
  (bind _returnvalue_2 (* (.effectiveness LaserInfo) _returnvalue))
  (bind _asbase_ship (Utilities|Casting|CastToBaseShip _hitactor))
  (bind _absorbed (Class|ILaserInterface|ReflectionEfficiency(Message) (Utilities|Array|Get(acopy) (Class|FunctionLibrary|GetPartsHitfromWorldLocation _impactpoint (Variables|/Script/Voidsinger.BaseShip|GetPartGrid _asbase_ship)))))
  (Niagara|SpawnSystematLocation "/Game/FX/Systems/NS_LaserEndPoint.NS_LaserEndPoint" (+ _impactpoint (* _impactnormal (/ (Class|PartGridComponent|GetPartGridScale (Variables|/Script/Voidsinger.BaseShip|GetPartGrid _asbase_ship)) -2.0))) (Math|Rotator|MakeRotator 0.0 0.0 (.yaw (Math|Conversions|RotationFromXVector _impactnormal))))
  (Class|PartGridComponent|ApplyHeatatLocation (Variables|/Script/Voidsinger.BaseShip|GetPartGrid _asbase_ship) (+ _impactpoint (* _impactnormal (/ (Class|PartGridComponent|GetPartGridScale (Variables|/Script/Voidsinger.BaseShip|GetPartGrid _asbase_ship)) -2.0))) (* (select (== _absorbed 0.0) 1.0 _absorbed) (* _returnvalue_2 (Variables|Default|GetHeatApplicationRate))))
  (Class|StarSystemLevelManager|ActivatewithEffects (CallFunction|GetStarSystemLevelManager) _hitactor (Class|BasePart|GetShip) (Class|FunctionLibrary|GetPartsHitfromWorldLocation (+ _impactpoint (* _impactnormal (/ (Class|PartGridComponent|GetPartGridScale (Variables|/Script/Voidsinger.BaseShip|GetPartGrid _asbase_ship)) -2.0))) (Variables|/Script/Voidsinger.BaseShip|GetPartGrid _asbase_ship)) _tracestart (+ _impactpoint (* _impactnormal (/ (Class|PartGridComponent|GetPartGridScale (Variables|/Script/Voidsinger.BaseShip|GetPartGrid _asbase_ship)) -2.0))) _returnvalue_2 0.0)
  (return))