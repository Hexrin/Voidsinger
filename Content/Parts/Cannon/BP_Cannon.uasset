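; BP_Cannon is a ship part that fires an explosive projectile when activated.
; Each tick it binds its Cannon event to the owning player ship.
; Firing draws one Ammo, but the success check is disconnected, so it always spawns a projectile.
; The spawn transform follows part offset and ship rotation, and the projectile receives the ship's velocity plus tangential speed derived from its spin.
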(event Custom|Cannon
  (params (Radius :type Float%20%28single-precision%29) (Velocity :type Float%20%28single-precision%29))
  (bind _returnvalue (Class|BasePart|GetPartRelativeLocation))
  (bind _returnvalue_2 (Class|BasePart|GetShip))
  (bind _returnvalue_3 (Transformation|GetActorRotation _returnvalue_2))
  (bind _physicscomponent (Variables|/Script/Voidsinger.BaseShip|GetPhysicsComponent _returnvalue_2))
  (bind _returnvalue_4 (Class|ShipPhysicsComponent|GetCenterOfMass _physicscomponent))
  ;[0.02064 1 0 1 12] Checks if the Canon has the needed resources to fire and removes one Ammo
  (bind _returnvalue_5 (Class|BaseResourceSystem|DrawResources (Class|BasePart|GetSystembyType "Ammo") 1.0))
  ;[1 1 1 1 12] Creates the Projectile and gets values for all of the variables
  (Game|SpawnActorfromClass "/Game/Parts/Cannon/CannonProjectile.CannonProjectile_C" (Math|Transform|MakeTransform (- (+ (+ (Transformation|GetActorLocation _returnvalue_2) _returnvalue_4) (Class|KismetMathLibrary|GetRotated2D (Math|Conversions|ToVector2D(Vector) (+ _returnvalue (Class|KismetMathLibrary|GetRotated2D (Variables|Default|GetOffset) (Class|BasePart|GetRelativeRotation)))) (.yaw (Transformation|GetActorRotation _returnvalue_2)))) _returnvalue_4) (Math|Rotator|MakeRotator (.roll _returnvalue_3) (.pitch _returnvalue_3) (+ (Class|BasePart|GetRelativeRotation) (.yaw _returnvalue_3))) "0.010000,0.010000,0.010000") "AlwaysSpawn" _returnvalue_2 Radius Velocity (Math|Conversions|ToVector(Vector2D) (Class|ShipPhysicsComponent|GetVelocity _physicscomponent)) (* (Math|Vector|Distance2D(Vector) _returnvalue_4 (Math|Conversions|ToVector2D(Vector) _returnvalue)) (Math|Trig|DegreesToRadians (Class|ShipPhysicsComponent|GetAngularVelocity _physicscomponent))) self 0))

(event EventBlueprintActivate
  (CallFunction|Cannon (Variables|Default|GetRadius) (Variables|Default|GetVelocity)))

(event EventOnTick
  (params (DeltaTime :type Float%20%28single-precision%29))
  ;[1 1 1 1 12] When Activated
  (bind _asbp_player_ship (Utilities|Casting|CastToBP_PlayerShip (Class|BasePart|GetShip)))
  (EventDispatchers|BindEventtoCannon _asbp_player_ship (delegate Custom|Cannon)))