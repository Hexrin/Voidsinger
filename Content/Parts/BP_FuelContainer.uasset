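; BP_FuelContainer is a part that contributes its StartingFuel amount to the Fuel system.
; On BeginPlay it gets that system by type and adds the amount as resources.
; On destruction it calls DrawResources with the negated amount to take the fuel back.
; If that draw fails, it lowers StartingFuel in fixed steps and retries until one succeeds, with no explicit lower bound.
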(event EventBeginPlay
  ;[0 0.3961 0.03922] The amount it adds should be a variable -Mabel
  (CallFunction|AddResources (CallFunction|GetSystembyType 0) (Variables|Default|GetStartingFuel)))

(event EventOnDestroyed
  (bind _returnvalue (CallFunction|DrawResources (CallFunction|GetSystembyType 0) (* (Variables|Default|GetStartingFuel) -1.0) :!label _label))
  (if (not _returnvalue)
    (Variables|Default|SetStartingFuel (- (Variables|Default|GetStartingFuel) 5e+01))
    (goto _label)))