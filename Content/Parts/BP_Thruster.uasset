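; BP_Thruster is a thruster part on a part grid, and its Blueprint graph only draws movement debug visuals.
; When MovementDebug is on in DebugSettings, each tick draws an arrow toward the thrust location, rotated in 2D by the grid owner's yaw and the thrust rotation.
; While thrusting, a larger, thicker red arrow is drawn over it.
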(event EventOnTick
  (params (DeltaTime :type Float%20%28single-precision%29))
  (bind _returnvalue (Class|BaseThrusterPart|GetThrustRotation))
  (bind _returnvalue_2 (Class|BaseThrusterPart|GetThrustLocation))
  (bind _returnvalue_3 (Class|BasePart|GetPartGrid))
  (bind _returnvalue_4 (Components|GetOwner _returnvalue_3))
  (bind _returnvalue_5 (Transformation|GetActorLocation _returnvalue_4))
  (bind _returnvalue_6 (Transformation|GetActorRotation _returnvalue_4))
  (bind _returnvalue_7 (Class|KismetMathLibrary|GetRotated2D _returnvalue_2 (.yaw _returnvalue_6)))
  (bind _returnvalue_8 (+ (.yaw _returnvalue_6) _returnvalue))
  (bind _returnvalue_9 (Class|KismetMathLibrary|GetRotated2D "(X=-1.500000,Y=0.000000)" _returnvalue_8))
  (bind _returnvalue_10 (+ _returnvalue_5 _returnvalue_7))
  (bind _returnvalue_11 (+ _returnvalue_10 _returnvalue_9))
  (if (.MovementDebug (Utilities|GetClassDefaults "/Game/DebugSettings.DebugSettings_C"))
    (Rendering|Debug|DrawDebugArrow _returnvalue_11 _returnvalue_10 0.25 "(R=1.000000,G=0.122685,B=0.000000,A=1.000000)" 0.0 0.1)
    (if (Class|BaseThrusterPart|IsThrusting)
      (Rendering|Debug|DrawDebugArrow _returnvalue_11 _returnvalue_10 0.5 "(R=1.000000,G=0.000000,B=0.000000,A=1.000000)" 0.0 0.2))))